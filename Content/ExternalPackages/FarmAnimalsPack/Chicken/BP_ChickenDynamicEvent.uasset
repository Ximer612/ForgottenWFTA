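; BP_ChickenDynamicEvent is a one-shot ambient event that sets a group of chickens running when the player enters a trigger.
; SchoolTrigger and PathTrigger share a HasTriggered guard and record whether the player came from the path.
; A recursive QueueChickens event passes that flag to each chicken's StartRunning, using a delay to stagger the starts evenly across TriggerDuration.
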(event OnComponentBeginOverlap(PathTrigger)
  (params (OverlappedComponent :type Primitive%20Component%20Object%20Reference) (OtherActor :type Actor%20Object%20Reference) (OtherComp :type Primitive%20Component%20Object%20Reference) (OtherBodyIndex :type Integer) (bFromSweep :type Boolean) (SweepResult :type Hit%20Result%20Structure%20%28by%20ref%29))
  (if (and (== OtherActor (Game|GetPlayerCharacter 0)) (not (Variables|Default|GetHasTriggered?)))
    (Variables|Default|SetHasTriggered? true)
    (Variables|Default|SetFromPath? true)
    (CallFunction|QueueChickens)))

(event OnComponentBeginOverlap(SchoolTrigger)
  (params (OverlappedComponent :type Primitive%20Component%20Object%20Reference) (OtherActor :type Actor%20Object%20Reference) (OtherComp :type Primitive%20Component%20Object%20Reference) (OtherBodyIndex :type Integer) (bFromSweep :type Boolean) (SweepResult :type Hit%20Result%20Structure%20%28by%20ref%29))
  (if (and (== OtherActor (Game|GetPlayerCharacter 0)) (not (Variables|Default|GetHasTriggered?)))
    (Variables|Default|SetHasTriggered? true)
    (Variables|Default|SetFromPath? false)
    (CallFunction|QueueChickens)))

(event Custom|QueueChickens
  (if (!= (Utilities|Array|Length (Variables|Default|GetChickens)) (Variables|Default|GetIndex))
    (Default|StartRunning (Utilities|Array|Get(acopy) (Variables|Default|GetChickens) (Variables|Default|GetIndex)) (Variables|Default|GetFromPath?))
    (Math|Integer|IncrementInt (Variables|Default|GetIndex)
      (:%20%20
        (Utilities|FlowControl|Delay (/ (Variables|Default|GetTriggerDuration) (Utilities|Array|Length (Variables|Default|GetChickens))))
        (CallFunction|QueueChickens)))))

(fn ConstructionScript)