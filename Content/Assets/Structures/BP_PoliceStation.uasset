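; BP_PoliceStation is a police station structure Blueprint that controls interior ambient sound for the player.
; Overlapping AudioTrigger1 starts and fades in InteriorSFX if it is not already playing.
; Leaving it fades out and stops the sound after a short delay, provided IsInside is false.
; IntTrigger1's overlap events are empty, and the logic that would set IsInside is disconnected, so this graph never updates that flag.
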(event OnComponentBeginOverlap(AudioTrigger1)
  (params (OverlappedComponent :type Primitive%20Component%20Object%20Reference) (OtherActor :type Actor%20Object%20Reference) (OtherComp :type Primitive%20Component%20Object%20Reference) (OtherBodyIndex :type Integer) (bFromSweep :type Boolean) (SweepResult :type Hit%20Result%20Structure%20%28by%20ref%29))
  (bind _interiorsfx (Variables|Default|GetInteriorSFX))
  (if (and (== OtherActor (Game|GetPlayerCharacter 0)) (not (Audio|Components|Audio|IsPlaying (Variables|Default|GetInteriorSFX))))
    (Audio|Components|Audio|Play _interiorsfx 0.0)
    (Audio|Components|Audio|FadeIn _interiorsfx 0.3 1.0 0.0 "Linear" :!class /Script/Engine.AudioComponent)))

(event OnComponentEndOverlap(AudioTrigger1)
  (params (OverlappedComponent :type Primitive%20Component%20Object%20Reference) (OtherActor :type Actor%20Object%20Reference) (OtherComp :type Primitive%20Component%20Object%20Reference) (OtherBodyIndex :type Integer))
  (bind _interiorsfx (Variables|Default|GetInteriorSFX))
  (if (Math|Boolean|ANDBoolean (Audio|Components|Audio|IsPlaying (Variables|Default|GetInteriorSFX)) (== (Game|GetPlayerCharacter 0) OtherActor) (not (Variables|Default|GetIsInside?)))
    (Audio|Components|Audio|StopDelayed _interiorsfx 0.3)
    (Audio|Components|Audio|FadeOut _interiorsfx 0.3 0.0 "Linear" :!class /Script/Engine.AudioComponent)))

(event OnComponentBeginOverlap(IntTrigger1)
  (params (OverlappedComponent :type Primitive%20Component%20Object%20Reference) (OtherActor :type Actor%20Object%20Reference) (OtherComp :type Primitive%20Component%20Object%20Reference) (OtherBodyIndex :type Integer) (bFromSweep :type Boolean) (SweepResult :type Hit%20Result%20Structure%20%28by%20ref%29)))

(event OnComponentEndOverlap(IntTrigger1)
  (params (OverlappedComponent :type Primitive%20Component%20Object%20Reference) (OtherActor :type Actor%20Object%20Reference) (OtherComp :type Primitive%20Component%20Object%20Reference) (OtherBodyIndex :type Integer)))

(fn ConstructionScript)