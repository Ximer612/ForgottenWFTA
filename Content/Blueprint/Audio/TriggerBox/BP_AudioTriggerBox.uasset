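; Trigger box actor that plays its audio while an actor tagged Player is inside.
; Begin overlap starts playback; end overlap runs a one-second fade, stopping the audio afterward only if the player has not re-entered.
; DestroyTrigger fades over a given duration, then destroys the actor; it sets IsDestroying to false, so that guard does not block re-triggering during the fade.
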(event OnComponentBeginOverlap(TriggerBox)
  (params (OverlappedComponent :type Primitive%20Component%20Object%20Reference) (OtherActor :type Actor%20Object%20Reference) (OtherComp :type Primitive%20Component%20Object%20Reference) (OtherBodyIndex :type Integer) (bFromSweep :type Boolean) (SweepResult :type Hit%20Result%20Structure%20%28by%20ref%29))
  (bind _audio (Variables|Default|GetAudio))
  (if (not (Variables|Default|GetIsDestroying?))
    (if (Actor|ActorHasTag OtherActor "Player")
      (Variables|Default|SetIsPlayerInside? true)
      (Components|Activation|Activate _audio false)
      (Audio|Components|Audio|Play _audio 0.0))))

(event OnComponentEndOverlap(TriggerBox)
  (params (OverlappedComponent :type Primitive%20Component%20Object%20Reference) (OtherActor :type Actor%20Object%20Reference) (OtherComp :type Primitive%20Component%20Object%20Reference) (OtherBodyIndex :type Integer))
  (if (Actor|ActorHasTag OtherActor "Player")
    (CallFunction|FadeandStopAudio 1.0)
    (Variables|Default|SetIsPlayerInside? false)))

(event Custom|FadeAndStopAudio
  (params (FadeOutDuration :type Float%20%28single-precision%29))
  (bind _audio (Variables|Default|GetAudio))
  (Audio|Components|Audio|FadeOut _audio FadeOutDuration 0.0 "Linear" :!class /Script/Engine.AudioComponent)
  (Utilities|FlowControl|Delay FadeOutDuration)
  (if (not (Variables|Default|GetIsPlayerInside?))
    (Audio|Components|Audio|Stop _audio)))

(event Custom|DestroyTrigger
  (params (FadeOutDuration :type Float%20%28single-precision%29))
  (Variables|Default|SetIsDestroying? false)
  (CallFunction|FadeandStopAudio FadeOutDuration)
  (Utilities|FlowControl|Delay FadeOutDuration)
  (Actor|DestroyActor))

(fn ConstructionScript)

(fn NewFunction)