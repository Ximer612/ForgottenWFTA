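; Town ambience manager that crossfades wind beds by player location and lantern state (present or past).
; BeginPlay spawns present outdoor and indoor loops; past-layer spawns are disabled, though switching still adjusts them.
; Looping timers trigger delayed, chance-based positional sounds: birds, dogs and flies around the player, or house creaks and thumps near HouseLocator.
; CanPlaySFX gates these sets oppositely; indoor locations and lantern changes clear it and pause the outdoor timer.
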(event Custom|CheckLocation
  (bind _fade_duration (Variables|Default|GetFade_Duration))
  (bind _fade_curve (Variables|Default|GetFade_Curve))
  (bind _fade_duration_2 (Variables|Default|GetFade_Duration))
  (bind _fade_curve_2 (Variables|Default|GetFade_Curve))
  (bind _randomsfxtimer (Variables|Default|GetRandomSFXTimer))
  (bind _amb_outdoor_present (Variables|Default|GetAmb_Outdoor_Present))
  (bind _amb_indoor_present (Variables|Default|GetAmb_indoor_Present))
  (bind _amb_indoor_past (Variables|Default|GetAmb_Indoor_Past))
  (bind _amb_outdoor_past (Variables|Default|GetAmb_Outdoor_Past))
  (if (not (Variables|Default|GetIs%20Lantern%20Enabled))
    ;[0.1373 0.1373 0.1373] IndoorSwitchPresent
    (switch int (Variables|Default|GetNewLocation)
      (:0
        (Audio|Components|Audio|AdjustVolume _amb_outdoor_present _fade_duration_2 1.0 _fade_curve_2 :!class /Script/Engine.AudioComponent)
        (Audio|Components|Audio|AdjustVolume _amb_indoor_present _fade_duration_2 0.001 _fade_curve_2 :!class /Script/Engine.AudioComponent)
        (Variables|Default|SetCurrentLocation 0)
        (Utilities|Time|UnpauseTimerbyHandle _randomsfxtimer)
        (Variables|Default|SetCanPlaySFX true))
      (:1
        (Audio|Components|Audio|AdjustVolume _amb_outdoor_present _fade_duration_2 0.001 _fade_curve_2 :!class /Script/Engine.AudioComponent)
        (Audio|Components|Audio|AdjustVolume _amb_indoor_present _fade_duration_2 1.0 _fade_curve_2 :!class /Script/Engine.AudioComponent)
        (Variables|Default|SetCurrentLocation 1)
        (Utilities|Time|PauseTimerbyHandle _randomsfxtimer :!label _label)
        (Variables|Default|SetCanPlaySFX false))
      (:2
        (Audio|Components|Audio|AdjustVolume _amb_outdoor_present _fade_duration_2 0.001 _fade_curve_2 :!class /Script/Engine.AudioComponent)
        (Audio|Components|Audio|AdjustVolume _amb_indoor_present _fade_duration_2 0.5 _fade_curve_2 :!class /Script/Engine.AudioComponent)
        (Variables|Default|SetCurrentLocation 2)
        (goto _label)))
    (Audio|Components|Audio|AdjustVolume (Variables|Default|GetAmb_Outdoor_Past) 1.0 0.001 "Linear" :!class /Script/Engine.AudioComponent)
    (Audio|Components|Audio|AdjustVolume (Variables|Default|GetAmb_Indoor_Past) 1.0 0.001 "Linear" :!class /Script/Engine.AudioComponent)
    (else
      ;[0.1373 0.1373 0.1373] IndoorSwitchPast
      (switch int (Variables|Default|GetNewLocation)
        (:0
          (Audio|Components|Audio|AdjustVolume _amb_outdoor_past _fade_duration 1.0 _fade_curve :!class /Script/Engine.AudioComponent)
          (Audio|Components|Audio|AdjustVolume _amb_indoor_past _fade_duration 0.001 _fade_curve :!class /Script/Engine.AudioComponent)
          (Variables|Default|SetCurrentLocation 0))
        (:1
          (Audio|Components|Audio|AdjustVolume _amb_outdoor_past _fade_duration 0.001 _fade_curve :!class /Script/Engine.AudioComponent)
          (Audio|Components|Audio|AdjustVolume _amb_indoor_past _fade_duration 1.0 _fade_curve :!class /Script/Engine.AudioComponent)
          (Variables|Default|SetCurrentLocation 1))
        (:2
          (Audio|Components|Audio|AdjustVolume _amb_outdoor_past _fade_duration 0.001 _fade_curve :!class /Script/Engine.AudioComponent)
          (Audio|Components|Audio|AdjustVolume _amb_indoor_past _fade_duration 0.001 _fade_curve :!class /Script/Engine.AudioComponent)
          (Variables|Default|SetCurrentLocation 2)))
      (Audio|Components|Audio|AdjustVolume (Variables|Default|GetAmb_Outdoor_Present) 1.0 0.001 "Linear" :!class /Script/Engine.AudioComponent)
      (Audio|Components|Audio|AdjustVolume (Variables|Default|GetAmb_indoor_Present) 1.0 0.001 "Linear" :!class /Script/Engine.AudioComponent))))

(event Custom|RandomSFXHouse
  (bind _houselocator (Variables|Default|GetHouseLocator))
  (bind _returnvalue (Transformation|GetActorLocation _houselocator))
  (Utilities|FlowControl|Sequence
    (:then_0
      ;[0.1373 0.1373 0.1373] SFX Random delay and chance
      (Utilities|FlowControl|Delay (Math|Random|RandomFloatinRange 2.0 8.0))
      (if (== (Math|Random|RandomIntegerinRange 0 1) 0)
        (if (not (Variables|Default|GetCanPlaySFX))
          (Audio|PlaySoundatLocation "/Game/Audio/SFX/SFX_Env/Misc/Wood/SFX_Env_WoodCreaking_Cue.SFX_Env_WoodCreaking_Cue" (+ _returnvalue (Math|Vector|MakeVector (Math|Random|RandomFloatinRange -4e+02 4e+02) (Math|Random|RandomFloatinRange -3.5e+02 3.5e+02) (Math|Random|RandomFloatinRange -2e+02 2e+02))) "0, 0, 0" 1.0 1.0 0.0 0 0 0 0))))
    (:then_1
      (Utilities|FlowControl|Delay (Math|Random|RandomFloatinRange 5.0 15.0))
      (if (== (Math|Random|RandomIntegerinRange 0 1) 0)
        (if (not (Variables|Default|GetCanPlaySFX))
          (Audio|PlaySoundatLocation "/Game/Audio/SFX/SFX_Env/Misc/Wood/SFX_Env_WoodThump_Cue.SFX_Env_WoodThump_Cue" (+ _returnvalue (Math|Vector|MakeVector (Math|Random|RandomFloatinRange -4e+02 4e+02) (Math|Random|RandomFloatinRange -3.5e+02 3.5e+02) (Math|Random|RandomFloatinRange -2e+02 2e+02))) "0, 0, 0" 1.0 1.0 0.0 0 0 0 0))))))

(event Custom|OnLanternActive
  (params (IsLanternEnabled :type Boolean))
  (bind _fade_duration (Variables|Default|GetFade_Duration))
  (bind _fade_curve (Variables|Default|GetFade_Curve))
  (bind _fade_duration_2 (Variables|Default|GetFade_Duration))
  (bind _fade_curve_2 (Variables|Default|GetFade_Curve))
  (bind _randomsfxtimer (Variables|Default|GetRandomSFXTimer))
  (bind _amb_outdoor_present (Variables|Default|GetAmb_Outdoor_Present))
  (bind _amb_indoor_present (Variables|Default|GetAmb_indoor_Present))
  (bind _amb_indoor_past (Variables|Default|GetAmb_Indoor_Past))
  (bind _amb_outdoor_past (Variables|Default|GetAmb_Outdoor_Past))
  (Variables|Default|SetIs%20Lantern%20Enabled IsLanternEnabled)
  (Utilities|Time|PauseTimerbyHandle (Variables|Default|GetRandomSFXTimer))
  (Variables|Default|SetCanPlaySFX false)
  (if (not (Variables|Default|GetIs%20Lantern%20Enabled))
    ;[0.1373 0.1373 0.1373] IndoorSwitchPresent
    (switch int (Variables|Default|GetNewLocation)
      (:0
        (Audio|Components|Audio|AdjustVolume _amb_outdoor_present _fade_duration_2 1.0 _fade_curve_2 :!class /Script/Engine.AudioComponent)
        (Audio|Components|Audio|AdjustVolume _amb_indoor_present _fade_duration_2 0.001 _fade_curve_2 :!class /Script/Engine.AudioComponent)
        (Variables|Default|SetCurrentLocation 0)
        (Utilities|Time|UnpauseTimerbyHandle _randomsfxtimer)
        (Variables|Default|SetCanPlaySFX true))
      (:1
        (Audio|Components|Audio|AdjustVolume _amb_outdoor_present _fade_duration_2 0.001 _fade_curve_2 :!class /Script/Engine.AudioComponent)
        (Audio|Components|Audio|AdjustVolume _amb_indoor_present _fade_duration_2 1.0 _fade_curve_2 :!class /Script/Engine.AudioComponent)
        (Variables|Default|SetCurrentLocation 1)
        (Utilities|Time|PauseTimerbyHandle _randomsfxtimer :!label _label)
        (Variables|Default|SetCanPlaySFX false))
      (:2
        (Audio|Components|Audio|AdjustVolume _amb_outdoor_present _fade_duration_2 0.001 _fade_curve_2 :!class /Script/Engine.AudioComponent)
        (Audio|Components|Audio|AdjustVolume _amb_indoor_present _fade_duration_2 0.5 _fade_curve_2 :!class /Script/Engine.AudioComponent)
        (Variables|Default|SetCurrentLocation 2)
        (goto _label)))
    (Audio|Components|Audio|AdjustVolume (Variables|Default|GetAmb_Outdoor_Past) 1.0 0.001 "Linear" :!class /Script/Engine.AudioComponent)
    (Audio|Components|Audio|AdjustVolume (Variables|Default|GetAmb_Indoor_Past) 1.0 0.001 "Linear" :!class /Script/Engine.AudioComponent)
    (else
      ;[0.1373 0.1373 0.1373] IndoorSwitchPast
      (switch int (Variables|Default|GetNewLocation)
        (:0
          (Audio|Components|Audio|AdjustVolume _amb_outdoor_past _fade_duration 1.0 _fade_curve :!class /Script/Engine.AudioComponent)
          (Audio|Components|Audio|AdjustVolume _amb_indoor_past _fade_duration 0.001 _fade_curve :!class /Script/Engine.AudioComponent)
          (Variables|Default|SetCurrentLocation 0))
        (:1
          (Audio|Components|Audio|AdjustVolume _amb_outdoor_past _fade_duration 0.001 _fade_curve :!class /Script/Engine.AudioComponent)
          (Audio|Components|Audio|AdjustVolume _amb_indoor_past _fade_duration 1.0 _fade_curve :!class /Script/Engine.AudioComponent)
          (Variables|Default|SetCurrentLocation 1))
        (:2
          (Audio|Components|Audio|AdjustVolume _amb_outdoor_past _fade_duration 0.001 _fade_curve :!class /Script/Engine.AudioComponent)
          (Audio|Components|Audio|AdjustVolume _amb_indoor_past _fade_duration 0.001 _fade_curve :!class /Script/Engine.AudioComponent)
          (Variables|Default|SetCurrentLocation 2)))
      (Audio|Components|Audio|AdjustVolume (Variables|Default|GetAmb_Outdoor_Present) 1.0 0.001 "Linear" :!class /Script/Engine.AudioComponent)
      (Audio|Components|Audio|AdjustVolume (Variables|Default|GetAmb_indoor_Present) 1.0 0.001 "Linear" :!class /Script/Engine.AudioComponent))))

(event Custom|AmbienceSFX
  (bind _returnvalue (Game|Player|GetPlayerPawn 0))
  (bind _canplaysfx (Variables|Default|GetCanPlaySFX))
  (bind _returnvalue_2 (Transformation|GetActorLocation _returnvalue))
  (Utilities|FlowControl|Sequence
    (:then_0
      ;[0.1373 0.1373 0.1373] SFX Random delay and chance
      (Utilities|FlowControl|Delay (Math|Random|RandomFloatinRange 5.0 1e+01))
      (if (== (Math|Random|RandomIntegerinRange 0 2) 0)
        (if _canplaysfx
          (Audio|PlaySoundatLocation "/Game/Audio/SFX/SFX_Env/Town/SFX_Env_Birds_CUE.SFX_Env_Birds_CUE" (+ _returnvalue_2 (Math|Vector|MakeVector (Utilities|RandomFloatPosNeg 8e+02 2e+03) (Utilities|RandomFloatPosNeg 8e+02 2e+03) (Math|Random|RandomFloatinRange 8e+02 2e+03))) "0, 0, 0" 1.0 1.0 0.0 0 0 0 0))))
    (:then_1
      (Utilities|FlowControl|Delay (Math|Random|RandomFloatinRange 5.0 15.0))
      (if (== (Math|Random|RandomIntegerinRange 0 3) 0)
        (if _canplaysfx
          (Audio|PlaySoundatLocation "/Game/Audio/SFX/SFX_Env/Town/SFX_Env_Dogs_CUE.SFX_Env_Dogs_CUE" (+ _returnvalue_2 (Math|Vector|MakeVector (Utilities|RandomFloatPosNeg 5e+03 8e+03) (Utilities|RandomFloatPosNeg 5e+03 8e+03) 0.0)) "0, 0, 0" 1.0 1.0 0.0 0 0 0 0))))
    (:then_2
      (Utilities|FlowControl|Delay (Math|Random|RandomFloatinRange 7.0 12.0))
      (if (== (Math|Random|RandomIntegerinRange 0 2) 0)
        (if _canplaysfx
          (Audio|PlaySoundatLocation "/Game/Audio/SFX/SFX_Env/Town/SFX_Env_Fly_CUE.SFX_Env_Fly_CUE" (+ _returnvalue_2 (Math|Vector|MakeVector (Utilities|RandomFloatPosNeg 0.0 2e+02) (Utilities|RandomFloatPosNeg 0.0 2e+02) 0.0)) "0, 0, 0" 1.0 1.0 0.0 0 0 0 0))))))

(event EventBeginPlay
  (bind _ambiencevolume_multiplier (Variables|Default|GetAmbienceVolume%20Multiplier))
  (Utilities|FlowControl|Sequence
    (:then_0
      (bind _returnvalue (Audio|SpawnSound2D "/Game/Audio/Ambience/Town/Amb_TownWind_Medium.Amb_TownWind_Medium" _ambiencevolume_multiplier 1.0 0.0 0))
      (bind _output_get (Variables|Default|SetAmb_Outdoor_Present _returnvalue))
      (Audio|Components|Audio|FadeIn _output_get 5.0 1.0 0.0 "SCurve" :!class /Script/Engine.AudioComponent)
      (Utilities|FlowControl|Sequence
        (:then_0
          (bind _returnvalue_2 (Utilities|Time|SetTimerbyEvent (delegate Custom|RandomSFXHouse) 1.0 true))
          (Variables|Default|SetRandomSFX _returnvalue_2))
        (:then_1
          (bind _returnvalue_3 (Utilities|Time|SetTimerbyEvent (delegate Custom|AmbienceSFX) 3.0 true))
          (Variables|Default|SetRandomSFXTimer _returnvalue_3))))
    (:then_1
      (bind _returnvalue_4 (Audio|SpawnSound2D "/Game/Audio/Ambience/Town/Amb_TownWind_Medium_Indoor.Amb_TownWind_Medium_Indoor" _ambiencevolume_multiplier 1.0 0.0 0))
      (bind _output_get_2 (Variables|Default|SetAmb_indoor_Present _returnvalue_4))
      (Audio|Components|Audio|FadeIn _output_get_2 1.0 0.002 0.0 "Linear" :!class /Script/Engine.AudioComponent))
    (:then_2
      (bind _returnvalue_5 (Audio|SpawnSound2D "/Game/Audio/Ambience/Town/Amb_TownPast.Amb_TownPast" _ambiencevolume_multiplier 1.0 0.0 0))
      (bind _output_get_3 (Variables|Default|SetAmb_Outdoor_Past _returnvalue_5))
      (Audio|Components|Audio|FadeIn _output_get_3 1.0 0.002 0.0 "Linear" :!class /Script/Engine.AudioComponent))
    (:then_3
      (bind _returnvalue_6 (Audio|SpawnSound2D "/Game/Audio/Ambience/Town/Amb_TownPast_Indoor.Amb_TownPast_Indoor" _ambiencevolume_multiplier 1.0 0.0 0))
      (bind _output_get_4 (Variables|Default|SetAmb_Indoor_Past _returnvalue_6))
      (Audio|Components|Audio|FadeIn _output_get_4 1.0 0.002 0.0 "Linear" :!class /Script/Engine.AudioComponent))))

(fn ConstructionScript)