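; Secret room music actor that plays a violin house theme while the player overlaps it.
; The first entry starts the track; later entries fade it back up with an S-curve.
; On exit it fades to near silence instead of stopping, so playback is never restarted.
; A Lantern event uses a FlipFlop to alternately add and clear submix effects.
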(event Custom|Lantern
  (Utilities|FlowControl|FlipFlop
    (:A
      (Class|AudioMixerBlueprintLibrary|AddSubmixEffect))
    (:B
      (Class|AudioMixerBlueprintLibrary|ClearSubmixEffects))))

(event Collision|EventActorBeginOverlap
  (params (OtherActor :type Actor%20Object%20Reference))
  (bind _housetheme_violin1 (Variables|Default|GetHouseTheme_Violin1))
  (if (Actor|ActorHasTag OtherActor "Player")
    (if (Variables|Default|GetPlaying)
      (Audio|Components|Audio|AdjustVolume _housetheme_violin1 3.0 1.0 "SCurve" :!class /Script/Engine.AudioComponent)
      (else
        (Audio|Components|Audio|Play _housetheme_violin1 0.0)
        (Variables|Default|SetPlaying true)))))

(event Collision|EventActorEndOverlap
  (params (OtherActor :type Actor%20Object%20Reference))
  (if (Actor|ActorHasTag OtherActor "Player")
    (Audio|Components|Audio|AdjustVolume (Variables|Default|GetHouseTheme_Violin1) 4.0 0.002 "SCurve" :!class /Script/Engine.AudioComponent)))

(fn ConstructionScript)