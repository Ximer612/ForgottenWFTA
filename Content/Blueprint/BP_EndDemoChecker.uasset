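; BP_EndDemoChecker is an actor that swaps level content once enough ghosts are completed, apparently to mark the end of the demo.
; On BeginPlay it hides the actors in ToEnableActors and turns off their collision.
; Each OnGhostComplete call increments a counter; on reaching GhostToComplete, it hides and destroys the ToDisableActors, then reveals the ToEnableActors and restores their collision.
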(event EventBeginPlay
  (for _array_element (Variables|Default|GetToEnableActors)
    (Rendering|SetActorHiddenInGame _array_element true)
    (Collision|SetActorEnableCollision _array_element false)))

(event EventOnGhostComplete
  (bind _result (Math|Integer|IncrementInt (Variables|Default|GetCurrentGhosts))
    (:%20%20
      (if (>= _result (Variables|Default|GetGhostToComplete))
        (for _array_element (Variables|Default|GetToDisableActors)
          (Rendering|SetActorHiddenInGame _array_element true)
          (Actor|DestroyActor _array_element))
        (for _array_element_2 (Variables|Default|GetToEnableActors)
          (Rendering|SetActorHiddenInGame _array_element_2 false)
          (Collision|SetActorEnableCollision _array_element_2 true))))))

(fn ConstructionScript)