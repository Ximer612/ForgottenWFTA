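; Scene-interaction component for a dirty grave that the player scrubs clean with the GraveBrush item.
; Mouse movement over the grave fades a dynamic decal material until a distance threshold marks it clean, then saves and queues optional dialogue.
; BeginPlay starts it clean if the ghost's DT_Ghosts name is already in the saved diary.
; The cursor switches between brush, lens and default, and clicking without the brush plays a cooldown-limited bark.
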(event Custom|PlayBark
  (if (Variables|Default|GetCanBark?)
    (Variables|Default|SetCanBark? false)
    (Utilities|PlayRandomBark (Variables|Default|GetDialogues%20Rown%20Name) 0.0)
    (Utilities|FlowControl|Delay (Variables|Default|GetTimeToPlayAnotherDialogue))
    (Variables|Default|SetCanBark? true)))

(event Input|EnhancedActionEvents|EnhancedInputActionIA_Look
  (params (ActionValue :type Vector%202D%20Structure) (ElapsedSeconds :type Float%20%28double-precision%29) (TriggeredSeconds :type Float%20%28double-precision%29) (InputAction :type Input%20Action%20Object%20Reference :default "/Game/Inputs/Actions/IA_Look.IA_Look"))
  (bind _returnvalue (Class|KismetMathLibrary|GetAbs2D ActionValue))
  (bind _dialogue_row_nameonclean (Variables|Default|GetDialogue%20Row%20NameOnClean))
  (bind (_x _y) (Math|Vector2D|BreakVector2D _returnvalue))
  (if (Math|Boolean|ANDBoolean (Variables|Default|GetHasBrush?) (Variables|Default|GetIsMouseColliding?) (not (Variables|Default|GetIsClean?)))
    (bind _output_get (Variables|Default|SetMouseMoveDistance (+ (Variables|Default|GetMouseMoveDistance) (+ _x _y))))
    (Rendering|Material|SetScalarParameterValue (Variables|Default|GetDirtyMaterial) "Opacity Intensity" (- 1.0 (/ _output_get (Variables|Default|GetMaxMouseDistance))) :!class /Script/Engine.MaterialInstanceDynamic)
    (bind _output_get_2 (Variables|Default|SetIsClean? (> _output_get (* (Variables|Default|GetMaxMouseDistance) 0.4))))
    (if _output_get_2
      (CallFunction|OnClickonMouseInteractionTrigger)
      (Class|ISaveable|SavetoGameData(Message) (Game|Player|GetPlayerPawn 0) true)
      (bind _isvalid_ (CallFunction|CheckValidRowName _dialogue_row_nameonclean))
      (if _isvalid_
        (Class|SNSNarrativeBlueprintFuncLib|EnqueueDialogue "/Game/Other/DataTables/Dialogues/DT_Items_Dialogues.DT_Items_Dialogues" _dialogue_row_nameonclean false)))))

(event EventBeginPlay
  (|CallParentFunction)
  (bind _returnvalue (Rendering|Material|CreateDynamicMaterialInstance (Variables|Default|GetDecal) :!class /Script/Engine.DecalComponent))
  (Variables|Default|SetDirtyMaterial _returnvalue)
  (bind _saveddata (Class|ISaveGame|GetGameData(Message) (Game|GetGameInstance)))
  (bind _returnvalue_2 (Utilities|GetDataTableRow "/Game/Other/DataTables/DT_Ghosts.DT_Ghosts" (Variables|Default|GetGhostRowName))
    (:then
      (if (Utilities|Array|ContainsItem (.FoundNameGhost (Utilities|Struct|BreakS_GhostsDiarySaveData (Variables|/Game/Blueprint/SaveGame/BP_GameData.BP_GameData_C|GetGhostsDiaryData _saveddata))) (Utilities|Struct|BreakS_GhostInfo _returnvalue_2))
        (Variables|Default|SetIsClean? true)
        (Rendering|Material|SetScalarParameterValue (Variables|Default|GetDirtyMaterial) "Opacity Intensity" 0.0 :!class /Script/Engine.MaterialInstanceDynamic)))
    (:RowNotFound
      (Development|PrintString "PLEASE SET A GHOST ROW NAME FOR A DIRTY GRAVE!" true true "(R=1.000000,G=0.000000,B=0.010551,A=1.000000)" 1e+01))))

(event EventInteract
  (params (LookingComponent :type Primitive%20Component%20Object%20Reference))
  (|CallParentFunction LookingComponent)
  (if (Variables|Default|GetIsClean?)
    (Variables|Default|SetHasBrush? true)
    (else
      (bind _hasitem_ (Class|IPlayerUtils|PlayerHasItem?(Message) (Game|Player|GetPlayerPawn 0) "GraveBrush"))
      (Variables|Default|SetHasBrush? _hasitem_))))

(fn ConstructionScript
  (|CallParentFunction))

(fn SetCursorInspection
  (bind _returnvalue (Game|GetPlayerController 0))
  (bind _hitresult (Game|Player|GetHitResultUnderCursorbyChannel _returnvalue "TraceTypeQuery3" true))
  (Utilities|IsValid (.hitcomponent _hitresult)
    (:Is%20Valid
      (if (and (.bblockinghit _hitresult) (Components|ComponentHasTag (.hitcomponent _hitresult) "ScenePointOfInterestTrigger"))
        (if (and (Variables|Default|GetHasBrush?) (not (Variables|Default|GetIsClean?)))
          (Class|WidgetBlueprintLibrary|SetHardwareCursor "Default" "T_CursorBrush" "(X=0.500000,Y=0.500000)")
          (else
            (Class|WidgetBlueprintLibrary|SetHardwareCursor "Default" "T_CursorLens" "(X=0.200000,Y=0.200000)")))
        (else
          (Class|WidgetBlueprintLibrary|SetHardwareCursor "Default" "T_WestCursor" "(X=0.000000,Y=0.000000)" :!label _label))))
    (:Is%20Not%20Valid
      (goto _label))))

(fn OnClickonMouseInteractionTrigger
  (params (ComponentClicked :type Actor%20Component%20Object%20Reference))
  (if (Variables|Default|GetHasBrush?)
    (if (Variables|Default|GetIsClean?)
      (|CallParentFunction 0))
    (else
      (CallFunction|PlayBark))))