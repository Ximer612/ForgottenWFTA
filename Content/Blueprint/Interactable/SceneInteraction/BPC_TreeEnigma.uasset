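; Scene interaction for the tree enigma, where the player saws through a rope to obtain a rope item.
; Clicking the trigger animates the saw into place, then horizontal look input slides it between two limits.
; Alternating strokes past each end play sounds and count cuts until a timeline drops the rope.
; The drop saves enigma completion and reveals the item; BeginPlay uses that saved flag to restore the solved state.
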(event Custom|MakeRopeFall
  (bind _returnvalue (Game|GetGameInstance))
  (bind _ropebottom (Variables|Default|GetROPEBOTTOM))
  (bind _relativelocation (Variables|/Script/Engine.SceneComponent|GetRelativeLocation _ropebottom))
  (Development|SetHiddeninGame (Variables|Default|GetGhostlyOverlay) true false) ; Hide Ghost Overlay
  (bind _alpha (Timeline|TL_FallingRope PlayFromStart) ; Animate falling rope
    (:Update
      (Transformation|SetRelativeLocation (Variables|Default|GetROPEBOTTOM) (Math|Vector|MakeVector (Math|Float|Lerp 125.0 3.5e+02 _alpha) (.y _relativelocation) (.z _relativelocation)) false false))
    (:Finished
      (Audio|PlaySound2D "/Game/Audio/SFX/SFX_Item/SFX_Items_RopeFalling.SFX_Items_RopeFalling" 1.0 1.0 0.0 0 0)
      (CallFunction|BacktoPlayerCamera)
      (bind _saveddata (Class|ISaveGame|GetGameData(Message) _returnvalue))
      (bind _structout (Utilities|Struct|SetmembersinS_EnigmasSaveData (Variables|/Game/Blueprint/SaveGame/BP_GameData.BP_GameData_C|GetEnigmasData _saveddata) true))
      (Class|ISaveGame|SaveEnigmasData(Message) _returnvalue true _structout)
      (Development|SetHiddeninGame (Variables|Default|GetROPEBOTTOM) true false)
      (Collision|SetCollisionEnabled (Variables|Default|GetInteractionBox) "NoCollision")
      (bind _ropeitembp (Variables|Default|GetRopeItemBP)
        (:then
          (Rendering|SetActorHiddenInGame _ropeitembp false)
          (Collision|SetActorEnableCollision _ropeitembp true))
        (:else
          (Development|PrintString "CANNOT CHANGE ROPE ITEM HIDDEN IN GAME PROPERTY"))))))

(event Custom|StartCutting
  (Development|SetHiddeninGame (Variables|Default|GetSaw) false false)
  (bind _movementalpha (Timeline|TL_MovingSaw PlayFromStart)
    (:Update
      (Transformation|SetRelativeLocation (Variables|Default|GetSaw) (Math|Vector|Lerp(Vector) "420.555592,9.585748,-5.674771" (Math|Vector|Lerp(Vector) (Variables|Default|GetMinSawLerpLocation) (Variables|Default|GetMaxSawLerpLocation) (Variables|Default|GetLerpSawValue)) _movementalpha) false false))))

(event Input|EnhancedActionEvents|EnhancedInputActionIA_Look
  (params (ActionValue :type Vector%202D%20Structure) (ElapsedSeconds :type Float%20%28double-precision%29) (TriggeredSeconds :type Float%20%28double-precision%29) (InputAction :type Input%20Action%20Object%20Reference :default "/Game/Inputs/Actions/IA_Look.IA_Look"))
  (bind _lerpsawvalue (Variables|Default|GetLerpSawValue))
  (bind _cutcounts (Variables|Default|GetCutCounts))
  (bind _lerpsawvalue_2 (Variables|Default|GetLerpSawValue))
  (CallFunction|CuttingRope ActionValue)
  (if (Variables|Default|GetIsFirstCut?)
    (if (> _lerpsawvalue_2 0.8)
      (Variables|Default|SetCuttingWay false)
      (Variables|Default|SetIsFirstCut? false :!label _label)
      (Utilities|FlowControl|FlipFlop :!label _label_2
        (:A
          ;[1 0 0] TODO: random sound + pitch with sound cue
          (Audio|PlaySound2D "/Game/Audio/SFX/SFX_Item/Saw/SFX_Items_Saw_Upstroke_Cue.SFX_Items_Saw_Upstroke_Cue" 1.0 1.0 0.0 0 0))
        (:B
          (Audio|PlaySound2D "/Game/Audio/SFX/SFX_Item/Saw/SFX_Items_Saw_Downstroke_Cue.SFX_Items_Saw_Downstroke_Cue" 1.0 1.0 0.0 0 0)))
      (Variables|Default|SetCuttingWay (not (Variables|Default|GetCuttingWay)))
      (Math|Integer|IncrementInt _cutcounts
        (:%20%20
          (if (> _cutcounts 4)
            (CallFunction|MakeRopeFall)
            (CallFunction|OnSceneInteractionCompleted))))
      (elif (< _lerpsawvalue_2 0.2)
        (Variables|Default|SetCuttingWay true)
        (goto _label)))
    (elif (Variables|Default|GetCuttingWay)
      (if (> _lerpsawvalue 0.8)
        (goto _label_2))
      (elif (< _lerpsawvalue 0.2)
        (goto _label_2)))))

(event EventInteract
  (params (LookingComponent :type Primitive%20Component%20Object%20Reference))
  (bind _hasitem_ (Class|IPlayerUtils|PlayerHasItem?(Message) (Game|Player|GetPlayerPawn 0) (Variables|Default|GetToUseItemRowName)))
  (Variables|Default|SetShouldLockMouse? _hasitem_)
  (|CallParentFunction 0))

(event EventBeginPlay
  (|CallParentFunction)
  (bind _saveddata (Class|ISaveGame|GetGameData(Message) (Game|GetGameInstance)))
  (if (Utilities|Struct|BreakS_EnigmasSaveData (Variables|/Game/Blueprint/SaveGame/BP_GameData.BP_GameData_C|GetEnigmasData _saveddata))
    (CallFunction|OnKeyItemAlreadyGot)
    (else
      (bind _ropeitembp (Variables|Default|GetRopeItemBP)
        (:then
          (Rendering|SetActorHiddenInGame _ropeitembp true)
          (Collision|SetActorEnableCollision _ropeitembp false))
        (:else
          (Development|PrintString "CANNOT CHANGE ROPE ITEM HIDDEN IN GAME PROPERTY"))))))

(fn ConstructionScript
  (|CallParentFunction))

(fn OnClickonMouseInteractionTrigger
  (params (ComponentClicked :type Actor%20Component%20Object%20Reference))
  (|CallParentFunction 0)
  (if (not (Variables|Default|GetIsCutting?))
    (Variables|Default|SetIsCutting? true)
    (CallFunction|StartCutting)))

(fn OnKeyItemAlreadyGot
  (|CallParentFunction)
  (Development|SetHiddeninGame (Variables|Default|GetROPEBOTTOM) true false)
  (Development|SetHiddeninGame (Variables|Default|GetSaw) true false)
  (Collision|SetCollisionEnabled (Variables|Default|GetInteractionBox) "NoCollision")
  (Development|SetHiddeninGame (Variables|Default|GetGhostlyOverlay) true false))

(fn CuttingRope
  (params (InVec :type Vector%202D%20Structure))
  (if (Variables|Default|GetIsCutting?)
    (Variables|Default|SetLerpSawValue (Math|Float|Clamp(Float) (+ (Variables|Default|GetLerpSawValue) (* (Math|Float|Sign(Float) (.X (Math|Vector2D|BreakVector2D InVec))) (Variables|Default|GetMouseSpeedMultiplier)))))
    (Transformation|SetRelativeLocation (Variables|Default|GetSaw) (Math|Vector|Lerp(Vector) (Variables|Default|GetMinSawLerpLocation) (Variables|Default|GetMaxSawLerpLocation) (Variables|Default|GetLerpSawValue)) false true)))