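; Master interactable door that swings on its pivot and starts locked when its key row name is valid.
; Interact toggles a timeline rotation if unlocked or the player has the key item, otherwise playing a locked sound; ForceOpen skips that check.
; LookAt reports lock state, while SetDoorStatus and OnGhostComplete can change it.
; Door sounds are pitch-randomized and throttled, and a construction-script arrow previews the opening angle.
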(event Custom|SetDoorStatus
  (params (NewStatus :type Boolean))
  (Variables|Default|SetIsLocked NewStatus))

(event Custom|PlaySound
  (params (SoundToPlay :type Sound%20Base%20Object%20Reference))
  ;[1 1 1] Add Impact SFX
  (Utilities|FlowControl|DoOnce false :!label _label
    (:Completed
      (Audio|SpawnSoundatLocation SoundToPlay (Transformation|GetActorLocation) "0, 0, 0" 1.0 (Math|Random|RandomFloatinRange 0.85 1.2) 0.0 "/Game/Audio/Settings/Attenuations/ATT_Audio3D.ATT_Audio3D" 0)
      (Utilities|FlowControl|Delay 0.4)
      (goto _label Reset))))

(event Custom|ForceOpen
  (Utilities|FlowControl|FlipFlop
    (:A
      (CallFunction|PlaySound "/Game/Audio/SFX/SFX_Env/Door/SFX_Env_Door_Close.SFX_Env_Door_Close")
      (bind _alpha (Timeline|TL_OpenDoor Play)
        (:Update
          (Transformation|SetRelativeRotation (Variables|Default|GetPivot) (Math|Rotator|Lerp(Rotator) (Variables|Default|GetCloseRotation) (Variables|Default|GetOpenRotation) _alpha true) false false))))
    (:B
      (CallFunction|PlaySound "/Game/Audio/SFX/SFX_Env/Door/SFX_Env_Door_Close_1.SFX_Env_Door_Close_1")
      (Timeline|TL_OpenDoor Reverse))))

(event EventInteract
  (params (LookingComponent :type Primitive%20Component%20Object%20Reference))
  (if (Variables|Default|GetIsLocked)
    (bind _hasitem_ (Class|IPlayerUtils|PlayerHasTakenItem?(Message) (Game|Player|GetPlayerPawn 0) (Variables|Default|GetKeyRowName)))
    (if _hasitem_
      (Utilities|FlowControl|FlipFlop :!label _label
        (:A
          (CallFunction|PlaySound "/Game/Audio/SFX/SFX_Env/Door/SFX_Env_Door_Close.SFX_Env_Door_Close")
          (bind _alpha (Timeline|TL_OpenDoor Play)
            (:Update
              (Transformation|SetRelativeRotation (Variables|Default|GetPivot) (Math|Rotator|Lerp(Rotator) (Variables|Default|GetCloseRotation) (Variables|Default|GetOpenRotation) _alpha true) false false))))
        (:B
          (CallFunction|PlaySound "/Game/Audio/SFX/SFX_Env/Door/SFX_Env_Door_Close_1.SFX_Env_Door_Close_1")
          (Timeline|TL_OpenDoor Reverse)))
      (else
        (Audio|PlaySoundatLocation "/Game/Audio/SFX/SFX_Misc/Door/SFX_DoorClosed.SFX_DoorClosed" (Transformation|GetActorLocation) "0, 0, 0" 1.0 1.0 0.0 "/Game/Audio/Settings/Attenuations/ATT_Audio3D.ATT_Audio3D" 0 0 0)))
    (else
      (goto _label))))

(event EventBeginPlay
  (bind _output_get (Variables|Default|SetCloseRotation (Variables|/Script/Engine.SceneComponent|GetRelativeRotation (Variables|Default|GetPivot))))
  (Variables|Default|SetOpenRotation (Math|Rotator|MakeRotator (.roll _output_get) (.pitch _output_get) (+ (.yaw _output_get) (Variables|Default|GetOpenDegree))))
  (bind _isvalid_ (CallFunction|CheckValidRowName (Variables|Default|GetKeyRowName)))
  (Variables|Default|SetIsLocked _isvalid_))

(event EventOnGhostComplete
  (Variables|Default|SetIsLocked false))

(fn ConstructionScript
  (Transformation|SetRelativeRotation (Variables|Default|GetArrow) (Math|Rotator|MakeRotator 0.0 0.0 (Variables|Default|GetOpenDegree)) false false))

(fn Lookat
  (params (Player%20Ref :type Actor%20Object%20Reference) (Hit%20Component :type Primitive%20Component%20Object%20Reference))
  (if (Variables|Default|GetIsLocked)
    (bind _hasitem_ (Class|IPlayerUtils|PlayerHasTakenItem?(Message) Player%20Ref (Variables|Default|GetKeyRowName)))
    (return Player%20Ref Hit%20Component "" (not _hasitem_))
    (else
      (return Player%20Ref Hit%20Component "" false))))