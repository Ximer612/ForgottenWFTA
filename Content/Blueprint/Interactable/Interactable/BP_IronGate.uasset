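; BP_IronGate is an interactable double iron gate that opens and closes, optionally locked behind a key item.
; Interact checks the player for the key or plays a random bark; SetDoorStatus and OnGhostComplete can change the lock.
; DoorSFX flip-flops between open and close sounds, driving a timeline forward or backward to lerp both pivots' yaw.
; LookAt reports the locked state, and PlaySound throttles pitch-randomized 3D audio.
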(event Custom|SetDoorStatus
  (params (NewStatus :type Boolean))
  ;[0.15 0.15 0.15 0.5] Initialize Variables
  (Variables|Default|SetIsLocked NewStatus))

(event Custom|PlaySound
  (params (SoundToPlay :type Sound%20Base%20Object%20Reference))
  ;[1 1 1] Add Impact SFX
  (Utilities|FlowControl|DoOnce false :!label _label
    (:Completed
      (Audio|SpawnSoundatLocation SoundToPlay (Transformation|GetActorLocation) "0, 0, 0" 1.0 (Math|Random|RandomFloatinRange 0.85 1.2) 0.0 "/Game/Audio/Settings/Attenuations/ATT_Audio3D.ATT_Audio3D" 0)
      (Utilities|FlowControl|Delay 0.4)
      (goto _label Reset))))

(event EventInteract
  (params (LookingComponent :type Primitive%20Component%20Object%20Reference))
  (bind _keyrowname (Variables|Default|GetKeyRowName))
  ;[0 0.15 0.04013 0.5] Interact Event
  (if (Variables|Default|GetIsLocked)
    (bind _isvalid_ (CallFunction|CheckValidRowName _keyrowname))
    (bind _hasitem_ (Class|IPlayerUtils|PlayerHasItem?(Message) (Game|Player|GetPlayerPawn 0) _keyrowname))
    (if (Math|Boolean|ANDBoolean _hasitem_ _isvalid_ (not (Variables|Default|GetInteracting?)))
      (Variables|Default|SetInteracting? true :!label _label)
      (Utilities|DoorSFX
        (:Opening
          (bind _alpha (Timeline|TL_OpenDoor Play)
            (:Update
              (CallFunction|SetDoorRotation _alpha))
            (:Finished
              (Variables|Default|SetInteracting? false))))
        (:Closing
          (Timeline|TL_OpenDoor Reverse)))
      (else
        (Utilities|PlayRandomBark (Variables|Default|GetDialogues%20Rown%20Name) (Variables|Default|GetTime%20to%20Play%20Dialogue))))
    (else
      (goto _label))))

(event EventBeginPlay
  ;[0.15 0.15 0.15 0.5] Initialize Variables
  (Components|Timeline|SetPlayRate (Variables|Default|GetTL_OpenDoor) (/ 1.0 (Variables|Default|GetTimelineLength))))

(event EventOnGhostComplete
  ;[0.15 0.15 0.15 0.5] Initialize Variables
  (Variables|Default|SetIsLocked false))

(fn ConstructionScript
  (Rendering|SetVisibility (Variables|Default|GetR_Pivot) false false))

(fn SetDoorRotation
  (params (Alpha :type Float%20%28single-precision%29))
  (bind _l_pivot (Variables|Default|GetL_Pivot))
  (bind _r_pivot (Variables|Default|GetR_Pivot))
  (bind _relativerotation (Variables|/Script/Engine.SceneComponent|GetRelativeRotation _r_pivot))
  (bind _relativerotation_2 (Variables|/Script/Engine.SceneComponent|GetRelativeRotation _l_pivot))
  (Transformation|SetRelativeRotation _l_pivot (Math|Rotator|MakeRotator (.roll _relativerotation_2) (.pitch _relativerotation_2) (Math|Float|Lerp (Variables|Default|GetL_StartRot) (Variables|Default|GetL_EndRot) Alpha)) false false)
  (Transformation|SetRelativeRotation _r_pivot (Math|Rotator|MakeRotator (.roll _relativerotation) (.pitch _relativerotation) (Math|Float|Lerp (Variables|Default|GetR_StartRot) (Variables|Default|GetR_EndRot) Alpha)) false false))

(fn SFXManager
  (params (StopAudio :type Audio%20Component%20Object%20Reference) (PlayAudio :type Sound%20Base%20Object%20Reference))
  (if (Audio|Components|Audio|IsPlaying StopAudio)
    (Audio|Components|Audio|Stop StopAudio))
  (bind _returnvalue (Audio|SpawnSoundatLocation PlayAudio (Transformation|GetActorLocation) "0, 0, 0" 1.0 1.0 0.0 0 0))
  (return _returnvalue))

(fn Lookat
  (params (Player%20Ref :type Actor%20Object%20Reference) (Hit%20Component :type Primitive%20Component%20Object%20Reference))
  (if (Variables|Default|GetIsLocked)
    (bind _hasitem_ (Class|IPlayerUtils|PlayerHasTakenItem?(Message) Player%20Ref (Variables|Default|GetKeyRowName)))
    (return Player%20Ref Hit%20Component "" (not _hasitem_))
    (else
      (return Player%20Ref Hit%20Component "" false))))