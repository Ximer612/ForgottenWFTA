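; Manager for the Abigail ghost hints that unlocks the ghost's cause of death in the player's diary.
; On BeginPlay it marks itself completed if saved diary data shows so, otherwise it checks whether every saved hint flag is set.
; UpdateHints saves each hint flag asynchronously and counts finds.
; When the count hits three, it queues optional all-hints dialogue, adds the diary entry and stops further updates.
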(event Custom|UpdateHints
  (params (ID :type Integer))
  (bind _returnvalue (Game|GetGameInstance))
  (bind _allhintsaudiorowname (Variables|Default|GetAllHintsAudioRowName))
  (if (not (Variables|Default|GetCompleted?))
    (bind _saveddata (Class|ISaveGame|GetGameData(Message) _returnvalue))
    (Utilities|Array|SetArrayElem (.triggerboxsubtitlesabigail (Variables|/Game/Blueprint/SaveGame/BP_GameData.BP_GameData_C|GetMapData _saveddata)) ID true true)
    (Class|ISaveGame|SaveMapData(Message) _returnvalue true (Variables|/Game/Blueprint/SaveGame/BP_GameData.BP_GameData_C|GetMapData _saveddata))
    (bind _result (Math|Integer|IncrementInt (Variables|Default|GetHintsFound))
      (:%20%20
        (if (== _result 3)
          (bind _isvalid_ (CallFunction|CheckValidRowName _allhintsaudiorowname))
          (if _isvalid_
            (Class|SNSNarrativeBlueprintFuncLib|EnqueueDialogue "/Game/Other/DataTables/Dialogues/DT_Trigger_Dialogues.DT_Trigger_Dialogues" _allhintsaudiorowname false))
          (Class|IPlayerUtils|AddDiaryGhostCauseOfDeath(Message) (Game|Player|GetPlayerPawn 0) (Variables|Default|GetGhostRowName))
          (Variables|Default|SetCompleted? true))))))

(event EventBeginPlay
  (bind _saveddata (Class|ISaveGame|GetGameData(Message) (Game|GetGameInstance)))
  (bind _returnvalue (Utilities|GetDataTableRow "/Game/Other/DataTables/DT_Ghosts.DT_Ghosts" (Variables|Default|GetGhostRowName))
    (:then
      (bind _completed_ (CallFunction|CheckifAbigailCompleted (.FoundGhostCurrentInfo (Utilities|Struct|BreakS_GhostsDiarySaveData (Variables|/Game/Blueprint/SaveGame/BP_GameData.BP_GameData_C|GetGhostsDiaryData _saveddata)))))
      (if (or _completed_ (Utilities|Array|ContainsItem (.FoundCauseOfDeathGhost (Utilities|Struct|BreakS_GhostsDiarySaveData (Variables|/Game/Blueprint/SaveGame/BP_GameData.BP_GameData_C|GetGhostsDiaryData _saveddata))) (.CauseOfDeath (Utilities|Struct|BreakS_GhostInfo _returnvalue))))
        (Variables|Default|SetCompleted? true)
        (else
          (CallFunction|CheckifAddHint))))))

(fn ConstructionScript)

(fn CheckifAddHint
  (bind _saveddata (Class|ISaveGame|GetGameData(Message) (Game|GetGameInstance)))
  (LocalVariables|SetAllTrue? true)
  (for _array_element (.TriggerBoxSubtitlesAbigail (Utilities|Struct|BreakS_MapSaveData (Variables|/Game/Blueprint/SaveGame/BP_GameData.BP_GameData_C|GetMapData _saveddata)))
    (if (not _array_element)
      (LocalVariables|SetAllTrue? false)
      (return)))
  (Variables|Default|SetCompleted? true)
  (Class|IPlayerUtils|AddDiaryGhostCauseOfDeath(Message) (Game|Player|GetPlayerPawn 0) (Variables|Default|GetGhostRowName)))

(fn CheckifAbigailCompleted
  (params (Array :type Array%20of%20S%20Ghost%20Save%20Data%20Structures))
  (for _array_element Array
    (if (== (.RowName (Utilities|Struct|BreakS_GhostSaveData _array_element)) (Variables|Default|GetGhostRowName))
      (return (.Completed? (Utilities|Struct|BreakS_GhostSaveData _array_element)))))
  (return false))