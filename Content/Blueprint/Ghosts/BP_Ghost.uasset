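; BP_Ghost is an interactable ghost NPC that plays dialogue and records itself in the player's diary.
; The first interaction plays an intro, reveals linked items and notifies actors; later ones cycle repeatable lines until the ghost is completed.
; Completion fires linked actors and trigger actions, saves the final-dialogue flag, then fades dynamic materials while Niagara smoke lerps to the player's lantern.
; Saved state hides finished ghosts on BeginPlay.
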(event Custom|LerpSmokeToPlayer
  (params (StartSmokeLocation :type Vector) (TargetSmokeLocation :type Vector))
  (bind _ns_ghostsmoke (Variables|Default|GetNS_GhostSmoke))
  (Components|Activation|Activate (Variables|Default|GetNS_GhostSmoke) false)
  (bind _alpha (Timeline|TL_MoveSmokeToPlayer PlayFromStart)
    (:Update
      (Transformation|SetWorldLocation _ns_ghostsmoke (Math|Vector|Lerp(Vector) StartSmokeLocation TargetSmokeLocation _alpha) false false)
      (Effects|Components|ParticleSystem|SetFloatParameter _ns_ghostsmoke "ScaleColor_Curve" (- 1.0 _alpha)))
    (:Finished
      (Components|Activation|Deactivate (Variables|Default|GetNS_GhostSmoke))
      (Audio|PlaySoundatLocation "/Game/Audio/SFX/SFX_Misc/Lantern/SFX_Env_DarknessSucc.SFX_Env_DarknessSucc" (Transformation|GetWorldLocation (Variables|Default|GetNS_GhostSmoke)) "0, 0, 0" 1.0 1.0 0.0 "/Game/Audio/Settings/Attenuations/ATT_Audio3D.ATT_Audio3D" 0 0 0))))

(event Custom|FadeGhost
  (CallFunction|SetPlayerMovements false)
  (Utilities|FlowControl|DoOnce false :!label _label
    (:Completed
      (CallFunction|TriggerDeathAnim)
      (Components|Activation|Deactivate (Variables|Default|GetNS_AuraGhost))
      (Components|Activation|Deactivate (Variables|Default|GetNS_Ghost_System))
      (bind _location (Class|IPlayerUtils|GetLanternActor(Message) (Game|Player|GetPlayerPawn 0)))
      (CallFunction|LerpSmoketoPlayer (Transformation|GetWorldLocation (Variables|Default|GetNS_GhostSmoke)) (Math|Vector|MakeVector (.x (Transformation|GetWorldLocation _location)) (.y (Transformation|GetWorldLocation _location)) (+ (.z (Transformation|GetWorldLocation _location)) 1e+01)))
      (bind _alpha (Timeline|TL_FadeGhost PlayFromStart)
        (:Update
          (for (_array_element _array_index) (Variables|Default|GetGhostMaterials)
            (Rendering|Material|SetScalarParameterValue _array_element (Variables|Default|GetMaterialParameterName) (Math|Float|Lerp (Utilities|Array|Get(acopy) (Variables|Default|GetGhostMaterialsValues) _array_index) 0.0 _alpha) :!class /Script/Engine.MaterialInstanceDynamic)
            (Development|PrintString (Utilities|String|ToString(Float) (Math|Float|Lerp (Utilities|Array|Get(acopy) (Variables|Default|GetGhostMaterialsValues) _array_index) 0.0 _alpha)))))
        (:Finished
          (Rendering|SetActorHiddenInGame true)
          (CallFunction|OnEndFading)
          (goto _label Reset))))))

(event Custom|TriggerDeathAnim)

(event Custom|AnimationEvent
  (bind _alpha (Timeline|TL_FadeGhost PlayFromStart)
    (:Update
      (for (_array_element _array_index) (Variables|Default|GetGhostMaterials)
        (Rendering|Material|SetScalarParameterValue _array_element (Variables|Default|GetMaterialParameterName) (Math|Float|Lerp (Utilities|Array|Get(acopy) (Variables|Default|GetGhostMaterialsValues) _array_index) 0.0 _alpha) :!class /Script/Engine.MaterialInstanceDynamic)
        (Development|PrintString (Utilities|String|ToString(Float) (Math|Float|Lerp (Utilities|Array|Get(acopy) (Variables|Default|GetGhostMaterialsValues) _array_index) 0.0 _alpha)))))
    (:Finished
      (Rendering|SetActorHiddenInGame true)
      (CallFunction|OnEndFading)
      (Utilities|FlowControl|DoOnce false) ; enters at Reset
    )))

(event Custom|Reverse%20Animation%20Event
  (for (_array_element _array_index) (Variables|Default|GetGhostMaterials)
    (Rendering|Material|SetScalarParameterValue _array_element (Variables|Default|GetMaterialParameterName) (Math|Float|Lerp (Utilities|Array|Get(acopy) (Variables|Default|GetGhostMaterialsValues) _array_index) 1.0 (stale Custom|FadeGhost _alpha)) :!class /Script/Engine.MaterialInstanceDynamic)))

(event Custom|RestorePlayerMovement
  (CallFunction|SetPlayerMovements false)
  (Class|IPlayerUtils|ShowOpenDiaryHint(Message) (Game|Player|GetPlayerPawn 0)))

(event EventBeginPlay
  (bind _isinsidesaves (Variables|Default|GetIsInsideSaves))
  (CallFunction|CreateDynamicMaterials)
  (bind (_amicompleted_ _lastdialogueplayed_) (CallFunction|CheckCompleted))
  (if (and _amicompleted_ _lastdialogueplayed_)
    (CallFunction|OnGhostCompleted false)
    (Rendering|SetActorHiddenInGame true)
    (if (Utilities|Array|IsNotEmpty (Variables|Customization|GetOnGhostCompleteActors))
      (Utilities|FlowControl|Delay 0.2)
      (CallFunction|OnGhostCompleted false))
    (else
      (Variables|Default|SetIsOneShotDialogue? (not _isinsidesaves))
      (if _isinsidesaves
        (CallFunction|SetMyItemsVisibility false)))))

(event EventInteract
  (params (LookingComponent :type Primitive%20Component%20Object%20Reference))
  (if (Variables|Default|GetCanInteract?)
    (Audio|PlaySound2D (Variables|Default|GetInteractSound) 1.0 1.0 0.0 0 0)
    (if (Variables|Default|GetIsOneShotDialogue?)
      (bind _playingaudio (CallFunction|PlayDialogue (Variables|Customization|GetIntroDialogueRowName) false))
      (Class|IPlayerUtils|BlockandWatchMe(Message) (Game|Player|GetPlayerPawn 0) self)
      (Class|SNSNarrativeBlueprintFuncLib|RegisterEventonEndDialogue _playingaudio false (delegate Custom|RestorePlayerMovement))
      (Variables|Default|SetLastPlayedDialogue _playingaudio)
      (Class|IPlayerUtils|AddDiaryGhost(Message) (Game|Player|GetPlayerPawn 0) (Variables|Customization|GetGhostRowName))
      (Variables|Default|SetIsOneShotDialogue? false)
      (for _array_element (Variables|Customization|GetOnGhostOneShotDialogueActors)
        (Class|IGhostable|OnGhostOneShotDialogue(Message) _array_element))
      (CallFunction|SetMyItemsVisibility true)
      (else
        (bind _amicompleted_ (CallFunction|CheckCompleted))
        (if (or _amicompleted_ (Variables|Default|GetIsCompleted?))
          (Class|IPlayerUtils|BlockandWatchMe(Message) (Game|Player|GetPlayerPawn 0) self)
          (bind _playingaudio_2 (CallFunction|PlayDialogue (Variables|Customization|GetCompletedDialogueRowName) false))
          (Variables|Default|SetLastPlayedDialogue _playingaudio_2)
          (CallFunction|OnGhostCompleted true)
          (Class|SNSNarrativeBlueprintFuncLib|RegisterEventonEndDialogue _playingaudio_2 false (delegate Custom|FadeGhost))
          (CallFunction|SetLastDialogue)
          (else
            (CallFunction|PlayDialogueinSequence)))))))

(fn ConstructionScript)

(fn PlayDialogue
  (params (AudioRowName :type Name) (StopAllOtherDialogues? :type Boolean))
  (bind _isvalid_ (CallFunction|CheckValidRowName AudioRowName))
  (if _isvalid_
    (Class|SNSNarrativeBlueprintFuncLib|EnqueueDialogue "/Game/Other/DataTables/Dialogues/DT_Ghosts_Dialogues.DT_Ghosts_Dialogues" AudioRowName StopAllOtherDialogues?)
    (Variables|Default|SetCanInteract? false)
    (Actor|Tick|SetActorTickEnabled true)
    (Collision|SetCollisionResponsetoChannel (Variables|Default|GetBox) "ECC_GameTraceChannel2" "ECR_Ignore")
    (Class|SNSNarrativeBlueprintFuncLib|RegisterEventonEndDialogue AudioRowName false (EventDispatchers|CreateEvent :!event ResetInteractable))
    (return AudioRowName)))

(fn CheckCompleted
  (bind _saveddata (Class|ISaveGame|GetGameData(Message) (Game|GetGameInstance)))
  (for _array_element (.foundghostcurrentinfo (Variables|/Game/Blueprint/SaveGame/BP_GameData.BP_GameData_C|GetGhostsDiaryData _saveddata))
    (if (== (Variables|Customization|GetGhostRowName) (.rowname _array_element))
      (Variables|Default|SetIsInsideSaves true)
      (return (.completed? _array_element) (.lastdialogueplayed? _array_element)))))

(fn PlayDialogueinSequence
  (bind _repeatabledialoguesrownames (Variables|Customization|GetRepeatableDialoguesRowNames))
  (if (> (Utilities|Array|Length _repeatabledialoguesrownames) 0)
    (CallFunction|PlayDialogue (Utilities|Array|Get(acopy) _repeatabledialoguesrownames (Variables|Default|GetNextDialogueIndex)) false)
    (Variables|Default|SetLastPlayedDialogue (Utilities|Array|Get(acopy) _repeatabledialoguesrownames (Variables|Default|GetNextDialogueIndex)))
    (Math|Integer|IncrementInt (Variables|Default|GetNextDialogueIndex)
      (:%20%20
        (Variables|Default|SetNextDialogueIndex (Math|Integer|%(Integer) (Variables|Default|GetNextDialogueIndex) (Utilities|Array|Length (Variables|Customization|GetRepeatableDialoguesRowNames))))
        (Collision|SetCollisionResponsetoChannel (Variables|Default|GetBox) "ECC_GameTraceChannel2" "ECR_Ignore")
        (return (Utilities|Array|Get(acopy) _repeatabledialoguesrownames (Variables|Default|GetNextDialogueIndex)))))))

(fn OnGhostCompleted
  (params (Audio? :type Boolean))
  (bind _onghostcompleteactors (Variables|Customization|GetOnGhostCompleteActors))
  (Utilities|FlowControl|Sequence
    (:then_0
      (if Audio?
        (Components|Activation|Activate (Variables|Default|GetNS_GhostSmoke) false)
        (Audio|PlaySound2D (Variables|Default|GetCompletedSound) 0.8 1.0 1.25 0 0 false))
      (Collision|SetActorEnableCollision false))
    (:then_1
      (for _array_element _onghostcompleteactors
        (Utilities|IsValid _array_element
          (:Is%20Valid
            (Class|IGhostable|OnGhostComplete(Message) _array_element)
            (Utilities|Array|RemoveItem _onghostcompleteactors _array_element)))))
    (:then_2
      (Variables|Default|SetIsCompleted? true)
      (Audio|Components|Audio|Stop (Variables|Default|GetSkeletalMesh)))
    (:then_3
      (for _array_element_2 (Variables|Default|GetTriggerActions)
        (Default|Event _array_element_2)))))

(fn ResetInteractable
  (Variables|Default|SetCanInteract? true)
  (Collision|SetCollisionResponsetoChannel (Variables|Default|GetBox) "ECC_GameTraceChannel2" "ECR_Block"))

(fn CreateDynamicMaterials
  (if (Utilities|Array|IsEmpty (Variables|Default|GetOriginalMaterials))
    (Variables|Default|SetOriginalMaterials (Rendering|Material|GetMaterials (Variables|Default|GetSkeletalMesh))))
  (Utilities|Array|Clear (Variables|Default|GetGhostMaterials))
  (for (_array_element _array_index) (Variables|Default|GetOriginalMaterials)
    (bind _returnvalue (Rendering|Material|CreateDynamicMaterialInstance _array_element "None" "None" :!class /Script/Engine.KismetMaterialLibrary))
    (Rendering|Material|SetMaterial (Variables|Default|GetSkeletalMesh) _array_index _returnvalue)
    (Utilities|Array|Add (Variables|Default|GetGhostMaterials) _returnvalue)
    (bind _returnvalue_2 (Rendering|Material|GetScalarParameterValue _returnvalue (Variables|Default|GetMaterialParameterName) :!class /Script/Engine.MaterialInstanceDynamic))
    (Utilities|Array|Add (Variables|Default|GetGhostMaterialsValues) _returnvalue_2)))

(fn OnEndFading)

(fn SetLastDialogue
  (bind _saveddata (Class|ISaveGame|GetGameData(Message) (Game|GetGameInstance)))
  (bind _output_get (LocalVariables|SetFoundGhostCurrentInfo (.FoundGhostCurrentInfo (Utilities|Struct|BreakS_GhostsDiarySaveData (Variables|/Game/Blueprint/SaveGame/BP_GameData.BP_GameData_C|GetGhostsDiaryData _saveddata)))))
  (for (_array_element _array_index) _output_get
    (if (== (.RowName (Utilities|Struct|BreakS_GhostSaveData _array_element)) (Variables|Customization|GetGhostRowName))
      (bind _structout (Utilities|Struct|SetmembersinS_GhostSaveData _array_element true))
      (Utilities|Array|SetArrayElem (LocalVariables|GetFoundGhostCurrentInfo) _array_index _structout)))
  (Class|ISaveGame|SaveGhostsData(Message) (Game|GetGameInstance) true (Utilities|Struct|MakeS_GhostsDiarySaveData _output_get (.FoundNameGhost (Utilities|Struct|BreakS_GhostsDiarySaveData (Variables|/Game/Blueprint/SaveGame/BP_GameData.BP_GameData_C|GetGhostsDiaryData _saveddata))) (.FoundCauseOfDeathGhost (Utilities|Struct|BreakS_GhostsDiarySaveData (Variables|/Game/Blueprint/SaveGame/BP_GameData.BP_GameData_C|GetGhostsDiaryData _saveddata))) (.FoundObjectGhost (Utilities|Struct|BreakS_GhostsDiarySaveData (Variables|/Game/Blueprint/SaveGame/BP_GameData.BP_GameData_C|GetGhostsDiaryData _saveddata))))))

(fn SetMyItemsVisibility
  (params (Visibile :type Boolean))
  (for _array_element (Variables|Default|GetMyItems)
    (Utilities|IsValid _array_element
      (:Is%20Valid
        (Collision|SetActorEnableCollision _array_element Visibile)
        (Rendering|SetActorHiddenInGame _array_element (not Visibile))))))

(fn IsInteractable
  (return true))