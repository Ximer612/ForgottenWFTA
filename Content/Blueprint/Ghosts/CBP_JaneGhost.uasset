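; Jane ghost Blueprint that handles her idle, interaction and death animation states, plus her completion after fading.
; A looping timer and a random IdleManager event drive idle variation, briefly pulsing the GhostState enum before resetting it.
; Interact pulses another state the same way, while TriggerDeathAnim sets one without reset.
; When fading ends, it notifies DemoChecker and queues a Timmy dialogue row; a delayed-restart graph also references TimmyAnims.
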(event Custom|IdleManager
  (switch int (Math|Random|RandomIntegerinRange 0 1)
    (:1
      (Variables|Default|SetGhostState "NewEnumerator1")
      (Utilities|FlowControl|Delay 0.1)
      (Variables|Default|SetGhostState "NewEnumerator0"))))

(event EventBeginPlay
  (|CallParentFunction)
  (bind _returnvalue (Utilities|Time|SetTimerbyEvent (EventDispatchers|CreateEvent :!event Custom|IdleManager) 1e+01 true true))
  (Variables|Default|SetAnimTimerHandle _returnvalue))

(event EventInteract
  (params (LookingComponent :type Primitive%20Component%20Object%20Reference))
  (|CallParentFunction LookingComponent)
  (Variables|Default|SetGhostState "NewEnumerator2")
  (Utilities|FlowControl|Delay 0.1)
  (Variables|Default|SetGhostState "NewEnumerator0"))

(event EventTriggerDeathAnim
  (Variables|Default|SetGhostState "NewEnumerator3"))

(fn ConstructionScript
  (|CallParentFunction))

(fn OnEndFading
  (|CallParentFunction)
  (Class|IGhostable|OnGhostComplete(Message) (Variables|Default|GetDemoChecker))
  (Class|SNSNarrativeBlueprintFuncLib|EnqueueDialogue "/Game/Other/DataTables/Dialogues/DT_Ghosts_Dialogues.DT_Ghosts_Dialogues" "Timmy_4" false))