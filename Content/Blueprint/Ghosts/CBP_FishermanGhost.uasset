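; Fisherman ghost Blueprint, a child ghost class that caches a boat reference and plays idle and activity animations.
; On BeginPlay it starts a randomized sitting loop that occasionally plays a looking montage between delays.
; Start events set fishing, card-playing, drinking or paddling states, with a cast montage for fishing and a repeating, randomly delayed drink montage.
; SetComponentState is empty, leaving the prop-switching logic for rod, bottle and oar disconnected.
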(event Custom|StartPlayingCards
  ;[0.15 0.15 0.15 0.5] Animation Events
  ;;[0.15 0.15 0.15 0.5] Start Playing Cards
  (Variables|Default|SetE_States "NewEnumerator1")
  (CallFunction|SetComponentState))

(event Custom|SittingAnims
  (switch int (Math|Random|RandomIntegerinRange 1 2)
    (:1
      _)
    (:2
      (Animation|Montage|PlayMontage (Variables|Default|GetSkeletalMesh) "/Game/Animations/NPC/Retargeted/AM_FishermanLooking.AM_FishermanLooking"
        (:OnCompleted
          _))))
  (Utilities|DelayandRestartAnims))

(event Custom|StartPaddling
  ;[0.15 0.15 0.15 0.5] Animation Events
  ;;[0.15 0.15 0.15 0.5] Start Paddling
  (Variables|Default|SetE_States "NewEnumerator2")
  (CallFunction|SetComponentState))

(event Custom|StartFishing
  ;[0.15 0.15 0.15 0.5] Animation Events
  ;;[0.15 0.15 0.15 0.5] Start Fishing
  (Variables|Default|SetE_States "NewEnumerator0")
  (CallFunction|SetComponentState)
  (Animation|Montage|PlayMontage (Variables|Default|GetSkeletalMesh) "/Game/Animations/NPC/MartinSmith/AM_FishingCast2.AM_FishingCast2"))

(event Custom|StartDrinking
  ;[0.15 0.15 0.15 0.5] Animation Events
  ;;[0.15 0.15 0.15 0.5] Start Drinking
  (Variables|Default|SetE_States "NewEnumerator3")
  (CallFunction|SetComponentState)
  (Animation|Montage|PlayMontage (Variables|Default|GetSkeletalMesh) "/Game/Animations/NPC/MartinSmith/AM_Drinking1.AM_Drinking1"
    (:OnCompleted
      (Utilities|FlowControl|Delay (Math|Random|RandomFloatinRange 3.0 8.0))
      (CallFunction|TakeDrink))))

(event Custom|SetComponentState
  ;[0.15 0.15 0.15 0.5] Set Component State
)

(event Custom|TakeDrink
  ;[0.15 0.15 0.15 0.5] Animation Events
  ;;[0.15 0.15 0.15 0.5] Start Drinking
  (Animation|Montage|PlayMontage (Variables|Default|GetSkeletalMesh) "/Game/Animations/NPC/MartinSmith/AM_Drinking1.AM_Drinking1"
    (:OnCompleted
      (Utilities|FlowControl|Delay (Math|Random|RandomFloatinRange 3.0 8.0))
      (CallFunction|TakeDrink))))

(event EventBeginPlay
  (|CallParentFunction)
  (CallFunction|SittingAnims)
  (bind _returnvalue (Actor|GetActorOfClass "/Game/Blueprint/Interactable/Interactable/CBP_Boat.CBP_Boat_C"))
  (Variables|Default|SetBoatRef _returnvalue))

(event EventOnGhostCompleted
  (params (Audio? :type Boolean))
  (|CallParentFunction Audio?))

(fn ConstructionScript
  (|CallParentFunction))

(fn DisableComponent
  (params (InputPin :type Static%20Mesh%20Component%20Object%20Reference))
  (Collision|SetCollisionEnabled InputPin "NoCollision")
  (Rendering|SetVisibility InputPin false false))

(fn EnableComponent
  (params (InputPin :type Static%20Mesh%20Component%20Object%20Reference))
  (Collision|SetCollisionEnabled InputPin "QueryAndPhysics")
  (Rendering|SetVisibility InputPin true false))