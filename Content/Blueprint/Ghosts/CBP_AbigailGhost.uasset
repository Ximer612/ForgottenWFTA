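; Abigail ghost Blueprint: an interactable NPC, while not hidden, that plays a reaction montage and then cries when talked to.
; While idle, it loops through randomly picked idle or look-around montages with random pauses.
; On BeginPlay it sets collision from save state and, a tick later, notifies two doors if the player has the Lantern message.
; TriggerDeathAnim sets a death-animation flag and sends staggered whisper messages to the player once.
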(event Custom|RandomizeIdle
  ;[0.15 0.15 0.15 0.5] Randomize Idle between Look Around/Look Distance/Idle
  (switch int (Math|Random|RandomIntegerinRange 1 3)
    (:2
      (Animation|Montage|PlayMontage (Variables|Default|GetSkeletalMesh) "/Game/Animations/NPC/Abigail/AM_LookAround1.AM_LookAround1"
        (:OnCompleted
          _)
        (:OnInterrupted
          _)))
    (:3
      (Animation|Montage|PlayMontage (Variables|Default|GetSkeletalMesh) "/Game/Animations/NPC/Abigail/AM_LookDistance1.AM_LookDistance1"
        (:OnCompleted
          _)
        (:OnInterrupted
          _))))
  (Utilities|FlowControl|Delay (Math|Random|RandomFloatinRange 5.0 15.0))
  (CallFunction|RandomizeIdle))

(event EventBeginPlay
  (|CallParentFunction)
  (Collision|SetActorEnableCollision (Variables|Default|GetIsInsideSaves))
  (CallFunction|RandomizeIdle)
  (Utilities|FlowControl|DelayUntilNextTick)
  (bind _hasitem_ (Class|IPlayerUtils|PlayerHasItem?(Message) (Game|Player|GetPlayerPawn 0) "Lantern"))
  (if _hasitem_
    (Class|IGhostable|OnGhostComplete(Message) (Variables|Default|GetTempDoorOutAbigail))
    (Class|IGhostable|OnGhostComplete(Message) (Variables|Default|GetTempDoorOtherDoor))))

(event EventInteract
  (params (LookingComponent :type Primitive%20Component%20Object%20Reference))
  ;[0.15 0.15 0.15 0.5] React when character talks to you the first time, then cry
  (if (not (Variables|Default|GetbHidden))
    (|CallParentFunction LookingComponent)
    (Animation|Montage|PlayMontage (Variables|Default|GetSkeletalMesh) "/Game/Animations/NPC/Abigail/AM_React1.AM_React1"
      (:OnCompleted
        (Animation|Montage|PlayMontage (Variables|Default|GetSkeletalMesh) "/Game/Animations/NPC/Abigail/AM_Crying.AM_Crying")))))

(event EventTriggerDeathAnim
  (Variables|Default|SetShouldPlayAnimDeath? true)
  (Utilities|FlowControl|DoOnce false
    (:Completed
      (Class|IPlayerUtils|AddWhisper(Message) (Game|Player|GetPlayerPawn 0) (Variables|Default|GetWhisper%20Row%20Name_1) 2)
      (Utilities|FlowControl|Delay 0.2)
      (Class|IPlayerUtils|AddWhisper(Message) (Game|Player|GetPlayerPawn 0) (Variables|Default|GetWhisper%20Row%20Name_2))
      (Utilities|FlowControl|Delay 0.2)
      (Class|IPlayerUtils|AddWhisper(Message) (Game|Player|GetPlayerPawn 0) (Variables|Default|GetWhisper%20Row%20Name_3)))))

(fn ConstructionScript
  (|CallParentFunction))

(fn IsInteractable
  (return (not (Variables|Default|GetbHidden))))