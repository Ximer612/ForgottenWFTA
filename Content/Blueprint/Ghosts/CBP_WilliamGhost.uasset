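; Ghost character Blueprint for William, extending a parent ghost class with a periodic idle animation and a follow-up when fading ends.
; A looping timer is set to trigger an idle action that pauses it, plays a sitting disbelief montage and unpauses it on completion.
; When fading ends, it notifies the DemoChecker that the ghost's message is complete and queues a Timmy dialogue line.
; Interaction is passed straight to the parent.
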(event Custom|WilliamAction
  (params (Action :type E_William_Actions%20Enum :default "NewEnumerator0"))
  (Utilities|Time|PauseTimerbyHandle (Variables|Default|GetAnimTimerHandle))
  (switch Utilities|FlowControl|Switch|SwitchonE_William_Actions Action
    (:NewEnumerator0
      (Animation|Montage|PlayMontage 0 "/Game/Animations/NPC/William/AM_William_Sitting_Disbelief.AM_William_Sitting_Disbelief"
        (:OnCompleted
          (Utilities|Time|UnpauseTimerbyHandle (Variables|Default|GetAnimTimerHandle)))))))

(event Custom|TimerDelegate_WilliamAction
  (CallFunction|WilliamAction "NewEnumerator0"))

(event EventBeginPlay
  (|CallParentFunction)
  (bind _returnvalue (Utilities|Time|SetTimerbyEvent (EventDispatchers|CreateEvent :!event Custom|TimerDelegate_WilliamAction) 1e+01 true false 1e+01))
  (Variables|Default|SetAnimTimerHandle _returnvalue))

(event EventInteract
  (params (LookingComponent :type Primitive%20Component%20Object%20Reference))
  (|CallParentFunction LookingComponent))

(fn ConstructionScript
  (|CallParentFunction))

(fn OnEndFading
  (|CallParentFunction)
  (Class|IGhostable|OnGhostComplete(Message) (Variables|Default|GetDemoChecker))
  (Class|SNSNarrativeBlueprintFuncLib|EnqueueDialogue "/Game/Other/DataTables/Dialogues/DT_Ghosts_Dialogues.DT_Ghosts_Dialogues" "Timmy_4" false))