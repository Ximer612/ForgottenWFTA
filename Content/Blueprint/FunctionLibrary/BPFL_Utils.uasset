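; Blueprint function library of shared helpers, mostly for styling UI buttons.
; Color getters feed functions that return text colors or plain colors from hover, focus or an override flag, with inverted and Whispers variants.
; GetBTNColor builds a button style on one border texture with a state-based tint.
; Other utilities validate row names, toggle player 0's move input, and move the mouse cursor by gamepad stick with a deadzone.
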(fn CheckValidRowName
  (params (RowName :type Name))
  (return (not (or (== RowName "") (== RowName "")))))

(fn GetUnselectedUIColor
  (return "(R=0.027451,G=0.062745,B=0.074510,A=1.000000)"))

(fn GetSelectedUIColor
  (return "(R=1.000000,G=1.000000,B=1.000000,A=1.000000)"))

(fn GetUnselectedInvertedUIColor
  (return "(R=0.000000,G=0.133333,B=0.176471,A=1.000000)"))

(fn GetBTNTextColor
  (params (MyButton :type Button%20Object%20Reference%20%28by%20ref%29) (OtherCheck :type Boolean))
  (if (Math|Boolean|ORBoolean (Widget|IsHovered MyButton) (Class|Widget|HasAnyUserFocus MyButton) OtherCheck)
    (return (Utilities|Struct|MakeSlateColor (CallFunction|GetSelectedUIColor) "UseColor_Specified"))
    (else
      (return (Utilities|Struct|MakeSlateColor (CallFunction|GetUnselectedUIColor) "UseColor_Specified")))))

(fn GetBTNColor
  (params (MyButton :type Widget%20Object%20Reference%20%28by%20ref%29) (OtherCheck :type Boolean))
  (if (Math|Boolean|ORBoolean (Widget|IsHovered MyButton) (Class|Widget|HasAnyUserFocus MyButton) OtherCheck)
    (LocalVariables|SetHoveredColor "(R=1.000000,G=1.000000,B=1.000000,A=1.000000)")
    (else
      (LocalVariables|SetHoveredColor "(R=0.043137,G=0.043137,B=0.043137,A=1.000000)")))
  (return (Utilities|Struct|MakeButtonStyle (Utilities|Struct|MakeSlateBrush (Utilities|Struct|MakeSlateColor (LocalVariables|GetHoveredColor) "UseColor_Specified") "Image" "NoTile" "NoMirror" "(X=32.000000,Y=32.000000)" "(Left=0.000000,Top=0.000000,Right=0.000000,Bottom=0.000000)" "/Game/Assets/Textures/UI/T_ItemSlotBorderBetter.T_ItemSlotBorderBetter" "(CornerRadii=(X=0.000000,Y=0.000000,Z=0.000000,W=0.000000),Color=(SpecifiedColor=(R=0.000000,G=0.000000,B=0.000000,A=0.000000),ColorUseRule=UseColor_Specified),Width=0.000000,RoundingType=HalfHeightRadius,bUseBrushTransparency=False)") (Utilities|Struct|MakeSlateBrush (Utilities|Struct|MakeSlateColor (LocalVariables|GetHoveredColor) "UseColor_Specified") "Image" "NoTile" "NoMirror" "(X=32.000000,Y=32.000000)" "(Left=0.000000,Top=0.000000,Right=0.000000,Bottom=0.000000)" "/Game/Assets/Textures/UI/T_ItemSlotBorderBetter.T_ItemSlotBorderBetter" "(CornerRadii=(X=0.000000,Y=0.000000,Z=0.000000,W=0.000000),Color=(SpecifiedColor=(R=0.000000,G=0.000000,B=0.000000,A=0.000000),ColorUseRule=UseColor_Specified),Width=0.000000,RoundingType=HalfHeightRadius,bUseBrushTransparency=False)") (Utilities|Struct|MakeSlateBrush (Utilities|Struct|MakeSlateColor (LocalVariables|GetHoveredColor) "UseColor_Specified") "Image" "NoTile" "NoMirror" "(X=32.000000,Y=32.000000)" "(Left=0.000000,Top=0.000000,Right=0.000000,Bottom=0.000000)" "/Game/Assets/Textures/UI/T_ItemSlotBorderBetter.T_ItemSlotBorderBetter" "(CornerRadii=(X=0.000000,Y=0.000000,Z=0.000000,W=0.000000),Color=(SpecifiedColor=(R=0.000000,G=0.000000,B=0.000000,A=0.000000),ColorUseRule=UseColor_Specified),Width=0.000000,RoundingType=HalfHeightRadius,bUseBrushTransparency=False)") "(TintColor=(SpecifiedColor=(R=1.000000,G=1.000000,B=1.000000,A=1.000000),ColorUseRule=UseColor_Specified),DrawAs=NoDrawType,Tiling=NoTile,Mirroring=NoMirror,ImageType=NoImage,ImageSize=(X=0.000000,Y=0.000000),Margin=(Left=0.000000,Top=0.000000,Right=0.000000,Bottom=0.000000),ResourceObject=None,OutlineSettings=(CornerRadii=(X=0.000000,Y=0.000000,Z=0.000000,W=0.000000),Color=(SpecifiedColor=(R=0.000000,G=0.000000,B=0.000000,A=0.000000),ColorUseRule=UseColor_Specified),Width=0.000000,RoundingType=HalfHeightRadius,bUseBrushTransparency=False),UVRegion=(Min=(X=0.000000,Y=0.000000),Max=(X=0.000000,Y=0.000000),bIsValid=False),bIsDynamicallyLoaded=False,ResourceName=\"\")" "(SpecifiedColor=(R=1.000000,G=0.000000,B=1.000000,A=1.000000),ColorUseRule=UseColor_Foreground)" "(SpecifiedColor=(R=1.000000,G=0.000000,B=1.000000,A=1.000000),ColorUseRule=UseColor_Foreground)" "(SpecifiedColor=(R=1.000000,G=0.000000,B=1.000000,A=1.000000),ColorUseRule=UseColor_Foreground)" "(SpecifiedColor=(R=1.000000,G=0.000000,B=1.000000,A=1.000000),ColorUseRule=UseColor_Foreground)" "(Left=0.000000,Top=0.000000,Right=0.000000,Bottom=0.000000)" "(Left=0.000000,Top=0.000000,Right=0.000000,Bottom=0.000000)" "(ResourceObject=None)" "(ResourceObject=None)")))

(fn GetBTNTextColorInverted
  (params (MyButton :type Button%20Object%20Reference%20%28by%20ref%29) (OtherCheck :type Boolean))
  (if (Math|Boolean|ORBoolean (Widget|IsHovered MyButton) (Class|Widget|HasAnyUserFocus MyButton) OtherCheck)
    (return (Utilities|Struct|MakeSlateColor (CallFunction|GetSelectedUIColor) "UseColor_Specified"))
    (else
      (return (Utilities|Struct|MakeSlateColor (CallFunction|GetUnselectedInvertedUIColor) "UseColor_Specified")))))

(fn GetGhostsBTNColor
  (params (MyButton :type Button%20Object%20Reference%20%28by%20ref%29) (OtherCheck :type Boolean))
  (bind _returnvalue (Widget|IsHovered MyButton))
  (bind _returnvalue_2 (Class|Widget|HasAnyUserFocus MyButton))
  (bind _returnvalue_3 (Math|Boolean|ORBoolean _returnvalue _returnvalue_2 OtherCheck))
  (if _returnvalue_3
    (return (CallFunction|GetSelectedUIColor) _returnvalue_3)
    (else
      (return (CallFunction|GetUnselectedUIColor) _returnvalue_3))))

(fn SetPlayerMovements
  (params (Disable? :type Boolean))
  (bind _returnvalue (Game|GetPlayerController 0))
  (if Disable?
    (Class|EnhancedInputLibrary|FlushPlayerInput _returnvalue)
    (Input|SetIgnoreMoveInput _returnvalue true)
    (else
      (Input|ResetIgnoreMoveInput _returnvalue))))

(fn GetGhostsBTNColorOnlyCheck
  (params (Check :type Boolean))
  (if Check
    (return (Utilities|Struct|MakeSlateColor (CallFunction|GetSelectedUIColor) "UseColor_Specified"))
    (else
      (return (Utilities|Struct|MakeSlateColor (CallFunction|GetUnselectedUIColor) "UseColor_Specified")))))

(fn GetBTNTextColorWhispers
  (params (MyButton :type Button%20Object%20Reference%20%28by%20ref%29) (OtherCheck :type Boolean))
  (if (Math|Boolean|ORBoolean (Widget|IsHovered MyButton) (Class|Widget|HasAnyUserFocus MyButton) OtherCheck)
    (return (Utilities|Struct|MakeSlateColor "(R=0.000000,G=0.000000,B=0.000000,A=1.000000)" "UseColor_Specified"))
    (else
      (return (Utilities|Struct|MakeSlateColor "(R=0.000000,G=0.000000,B=0.000000,A=0.750000)" "UseColor_Specified")))))

(fn MoveMousewithGamepad
  (params (CanGamepadMoveMouse? :type Boolean) (MouseActionValue :type Vector%202D%20Structure) (PlayerController :type Player%20Controller%20Object%20Reference))
  (bind (_x _y) (Math|Vector2D|BreakVector2D MouseActionValue))
  (bind (_x_2 _y_2) (Math|Vector2D|BreakVector2D MouseActionValue))
  (bind (_locationx _locationy) (Game|Player|GetMousePosition PlayerController))
  (bind _joypadrotationdeadzone (LocalVariables|GetJoypadRotationDeadzone))
  (if (and CanGamepadMoveMouse? (or (> (Math|Float|Absolute(Float) _x_2) _joypadrotationdeadzone) (> (Math|Float|Absolute(Float) _y_2) _joypadrotationdeadzone)))
    (Class|PlayerController|SetMouseLocation PlayerController (Math|Float|Round (+ (* _x (LocalVariables|GetMouseMovementMultiplier)) _locationx)) (Math|Float|Round (+ (* _y (* (LocalVariables|GetMouseMovementMultiplier) -1.0)) _locationy)))))