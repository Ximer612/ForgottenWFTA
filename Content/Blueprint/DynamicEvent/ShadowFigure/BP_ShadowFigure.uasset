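; BP_ShadowFigure is a dynamic-event actor for a shadow figure that vanishes once triggered.
; Activate hides the JJJ component and its children, starts the SmokeFallof effect and records the actor through the BPCSaveable component.
; On BeginPlay it destroys itself if that component finds it in saves, so a triggered figure does not reappear.
; The construction script makes the whole component hierarchy visible.
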(event EventActivate
  (Rendering|SetVisibility (Variables|Default|GetJJJ) false true)
  (Components|Activation|Activate (Variables|Default|GetSmokeFallof) false)
  (Default|AddtoSaves (Variables|Default|GetBPC_Saveable)))

(event EventBeginPlay
  (bind _found_ (Default|CheckFoundinSaves (Variables|Default|GetBPC_Saveable)))
  (if _found_
    (Actor|DestroyActor)))

(fn ConstructionScript
  (Rendering|SetVisibility (Variables|Default|GetDefaultSceneRoot) true true))