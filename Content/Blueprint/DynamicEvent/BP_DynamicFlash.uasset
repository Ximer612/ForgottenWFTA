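; BP_DynamicFlash is a dynamic-event light effect that flashes a spotlight and a matching ray when activated.
; BeginPlay applies one shared color to the SpotLight and the Ray's materials, while construction starts the ray fully transparent.
; Activate plays the Flicker timeline, whose alpha curve scales both light intensity and ray opacity from zero to their set maximums.
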(event EventBeginPlay
  (bind _lightcolor (Variables|Default|GetLightColor))
  (Rendering|Components|Light|SetLightColor (Variables|Default|GetSpotLight) _lightcolor true)
  (Rendering|Material|SetVectorParameterValueonMaterials (Variables|Default|GetRay) "Color" (Math|Conversions|ToVector(LinearColor) _lightcolor)))

(event EventActivate
  (bind _alphacurve (Timeline|Flicker Play)
    (:Update
      (Rendering|Components|Light|SetIntensity (Variables|Default|GetSpotLight) (Math|Float|Lerp 0.0 (Variables|Default|GetIntensity) _alphacurve))
      (Rendering|Material|SetScalarParameterValueonMaterials (Variables|Default|GetRay) "Opacity" (Math|Float|Lerp 0.0 (Variables|Default|GetMaxOpacity) _alphacurve)))))

(fn ConstructionScript
  (Rendering|Material|SetScalarParameterValueonMaterials (Variables|Default|GetRay) "Opacity" 0.0))