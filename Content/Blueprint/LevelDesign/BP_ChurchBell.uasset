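; BP_ChurchBell is a level actor that rings a church bell on the quarter hours of the real-world clock.
; A looping timer started at BeginPlay checks the current minute every ten seconds and plays the bell cue at the actor's location with large-radius town ambience attenuation.
; A Playing flag held through a one-minute delay prevents repeated rings within the same minute.
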(event Custom|StartBellTimer
  (Utilities|Time|SetTimerbyEvent (delegate Custom|CheckTime) 1e+01 true))

(event Custom|CheckTime
  (bind _returnvalue (Math|DateTime|Now))
  (bind _returnvalue_2 (Class|KismetMathLibrary|GetMinute _returnvalue))
  (if (not (Variables|Default|GetPlaying?))
    (if (Math|Boolean|ORBoolean (== _returnvalue_2 0) (== _returnvalue_2 15) (== _returnvalue_2 30) (== _returnvalue_2 45))
      (Variables|Default|SetPlaying? true)
      (Audio|PlaySoundatLocation "/Game/Audio/SFX/SFX_Env/Church/SC_ChurchBell.SC_ChurchBell" (Transformation|GetActorLocation self) "0, 0, 0" 1.0 1.0 0.0 "/Game/Audio/Ambience/Town/SA_TownAmbience_LargeRadius.SA_TownAmbience_LargeRadius" 0 0 0)
      (Utilities|FlowControl|Delay 6e+01)
      (Variables|Default|SetPlaying? false))))

(event EventBeginPlay
  (CallFunction|StartBellTimer))

(fn ConstructionScript)