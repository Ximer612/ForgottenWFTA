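; Level design actor that plays a configured Level Sequence when its event is triggered.
; The event creates a sequence player and starts playback, with a DoOnce flag that can limit it to a single run.
; A saveable component gets a random GUID in the construction script, and the actor destroys itself on BeginPlay if that component is already in the saves.
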(event EventBeginPlay
  (if (Variables|/Game/Blueprint/Components/BPC_Saveable.BPC_Saveable_C|GetIsInSaves? (Variables|Default|GetBPC_Saveable))
    (Actor|DestroyActor)))

(event EventEvent
  (if (Variables|Default|GetDoOnce?)
    (Utilities|FlowControl|DoOnce false
      (:Completed
        _)))
  (bind _returnvalue (Sequencer|Player|CreateLevelSequencePlayer (Variables|Default|GetLevelSequece)))
  (Sequencer|Player|Play _returnvalue :!class /Script/MovieScene.MovieSceneSequencePlayer))

(fn ConstructionScript
  (|CallParentFunction)
  (Default|GenerateRandomGUID (Variables|Default|GetBPC_Saveable)))