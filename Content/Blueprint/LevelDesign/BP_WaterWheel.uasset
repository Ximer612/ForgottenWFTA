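; Water wheel level-design actor that keeps its mechanism mesh rotating continuously from BeginPlay.
; Each cycle captures the mesh's relative rotation, adds RotationAmount to pitch, and lerps toward it with the StuckWheelRotation timeline's alpha.
; The timeline's Finished event starts the next step, and its play rate is the inverse of AnimationSeconds.
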(event Custom|RotateWaterWheel
  (bind _output_get (Variables|Default|SetStartRot (Variables|/Script/Engine.SceneComponent|GetRelativeRotation (Variables|Default|GetSM_WheelMechanism_01a))))
  (Variables|Default|SetEndRot (Math|Rotator|MakeRotator (.roll _output_get) (+ (.pitch _output_get) (Variables|Default|GetRotationAmount)) (.yaw _output_get)))
  (bind _rotationalpha (Timeline|StuckWheelRotation PlayFromStart)
    (:Update
      (Transformation|SetRelativeRotation (Variables|Default|GetSM_WheelMechanism_01a) (Math|Rotator|Lerp(Rotator) (Variables|Default|GetStartRot) (Variables|Default|GetEndRot) _rotationalpha) false false))
    (:Finished
      (CallFunction|RotateWaterWheel))))

(event EventBeginPlay
  (CallFunction|RotateWaterWheel)
  (Components|Timeline|SetPlayRate (Variables|Default|GetStuckWheelRotation) (/ 1.0 (Variables|Default|GetAnimationSeconds))))

(fn ConstructionScript)