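; BP_OpenClose_Door is a level-design Blueprint that opens, closes or locks a referenced door when its custom event fires.
; Without Lock, the event toggles DoorToInteract based on its IsOpen state.
; With Lock set, it closes the door if open, then calls SetDoorStatus(true) on it, and never opens it.
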(event EventBeginPlay
  (|CallParentFunction) ; This node is disabled and will not be called.\nDrag off pins to build functionality.
)

(event Collision|EventActorBeginOverlap
  (params (OtherActor :type Actor%20Object%20Reference))
  (|CallParentFunction OtherActor) ; This node is disabled and will not be called.\nDrag off pins to build functionality.
)

(event EventTick
  (params (DeltaSeconds :type Float%20%28single-precision%29))
  (|CallParentFunction DeltaSeconds) ; This node is disabled and will not be called.\nDrag off pins to build functionality.
)

(event EventEvent
  (bind _doortointeract (Variables|Default|GetDoorToInteract))
  (bind _lock_ (Variables|Default|GetLock?))
  (if (Variables|/Game/Blueprint/Interactable/Interactable/BP_Door.BP_Door_C|GetIsOpen? _doortointeract)
    (if _lock_
      (Default|Close _doortointeract)
      (Default|SetDoorStatus _doortointeract true :!label _label)
      (else
        (Default|Close _doortointeract)))
    (elif _lock_
      (goto _label)
      (else
        (Default|Open _doortointeract)))))

(fn ConstructionScript
  (|CallParentFunction))