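; Debug variant of a one-shot level trigger box that runs a list of trigger actions and persists its used state through the save system.
; The first actor overlap while active adds it to saves via BPCSaveable, calls Event on each TriggerAction entry, then deactivates it.
; BPCSaveable gets a random GUID in the construction script; when found in saves, the trigger destroys itself and prints a debug message.
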(event Custom|InSaves
  (Actor|DestroyActor)
  (Development|PrintString "Dovrei distruggermi"))

(event EventBeginPlay
  (EventDispatchers|BindEventtoOnFoundinSaves (Variables|Default|GetBPC_Saveable) (delegate Custom|InSaves)))

(event Collision|EventActorBeginOverlap
  (params (OtherActor :type Actor%20Object%20Reference))
  (if (Variables|Default|GetIsActive?)
    (Default|AddtoSaves (Variables|Default|GetBPC_Saveable))
    (for _array_element (Variables|Default|GetTriggerAction)
      (Default|Event _array_element))
    (Variables|Default|SetIsActive? false)))

(fn ConstructionScript
  (Default|GenerateRandomGUID (Variables|Default|GetBPC_Saveable)))