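; Cursed lantern prop that starts dark and lights up through player interaction, an external light activation or ghost completion.
; Activation enables Tick, which lerps smoke to the player's lantern, then notifies warp boxes and fades the light in via timeline.
; Interacting also arms a trigger box and plays ghost dialogue and a whisper.
; BPCSaveable records activation, restoring the lit, non-interactive state on load.
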(event Custom|InSaves!
  (CallFunction|SetLightVisibility true)
  (Variables|Default|SetIsLightAlreadyVisible? true)
  (Collision|SetCollisionProfileName (Variables|Default|GetTriggerCollision) "NoCollision" true :!class /Script/Engine.PrimitiveComponent)
  (Actor|Tick|SetActorTickEnabled false)
  (Rendering|Material|SetMaterial (Variables|Default|GetStaticMesh) 0 "/Game/ExternalPackages/WesterTown/Materials/Props/MI_Lantern.MI_Lantern")
  (Components|Activation|Deactivate (Variables|Default|GetNiagara))
  (Collision|SetActorEnableCollision false)
  (Components|DestroyComponent (Variables|Default|GetStaticMesh1)))

(event Custom|NotInSaves!
  (CallFunction|SetLightVisibility false)
  (Audio|Components|Audio|Stop (Variables|Default|GetCracklingAudio)))

(event EventBeginPlay
  (bind _bpc_saveable (Variables|Default|GetBPC_Saveable))
  (EventDispatchers|BindEventtoOnFoundinSaves _bpc_saveable (delegate Custom|InSaves!))
  (EventDispatchers|BindEventtoOnNotinSaves _bpc_saveable (delegate Custom|NotInSaves!))
  (Default|CheckFoundinSaves _bpc_saveable)
  (Variables|Default|SetIntensity (Variables|/Script/Engine.LightComponentBase|GetIntensity (Variables|Default|GetPointLight))))

(event EventTick
  (params (DeltaSeconds :type Float%20%28single-precision%29))
  (if (Variables|Default|GetIsLightAlreadyVisible?)
    (Actor|Tick|SetActorTickEnabled false :!label _label)
    (Components|Activation|Deactivate (Variables|Default|GetSmoke))
    (for _array_element (Variables|Default|GetWarpBoxes)
      (Class|ILightningPole|OnLightActivation(Message) _array_element))
    (if (Variables|Default|GetIsLightAlreadyVisible?)
      _
      (else
        (Audio|PlaySoundatLocation "/Game/Audio/SFX/SFX_Misc/Lantern/SFX_Env_DarknessSucc.SFX_Env_DarknessSucc" (Transformation|GetWorldLocation (Variables|Default|GetSmoke)) "0, 0, 0" 1.0 1.0 0.0 "/Game/Audio/Settings/Attenuations/ATT_Audio3D.ATT_Audio3D" 0 0 0)
        (Audio|PlaySoundatLocation "/Game/Audio/SFX/SFX_Misc/Lantern/SFX_Env_FireStart_Cue.SFX_Env_FireStart_Cue" (Transformation|GetWorldLocation (Variables|Default|GetFire)) "0, 0, 0" 1.0 1.0 0.0 "/Game/Audio/Settings/Attenuations/ATT_Audio3D.ATT_Audio3D" 0 0 0)))
    (Rendering|Components|Light|SetIntensity (Variables|Default|GetPointLight) 0.0)
    (CallFunction|SetLightVisibility true)
    (bind _alpha (Timeline|TL_LanternLightOn PlayFromStart)
      (:Update
        (Rendering|Components|Light|SetIntensity (Variables|Default|GetPointLight) (* _alpha (Variables|Default|GetIntensity))))
      (:Finished
        (Components|DestroyComponent (Variables|Default|GetSmoke))))
    (else
      (bind _location (Class|IPlayerUtils|GetLanternActor(Message) (Game|Player|GetPlayerPawn 0)))
      (bind _output_get (Variables|Default|SetGoToPlayerCounter (+ DeltaSeconds (Variables|Default|GetGoToPlayerCounter))))
      (Transformation|SetWorldLocation (Variables|Default|GetSmoke) (Math|Vector|Lerp(Vector) (Transformation|GetWorldLocation (Variables|Default|GetPointLight)) (Transformation|GetWorldLocation _location) (/ _output_get (Variables|Default|GetGoToPlayerTimer))) false false)
      (if (> (Variables|Default|GetGoToPlayerCounter) (Variables|Default|GetGoToPlayerTimer))
        (goto _label)))))

(event EventOnLightActivation
  (Utilities|ActivateLightingPole))

(event EventInteract
  (params (LookingComponent :type Primitive%20Component%20Object%20Reference))
  (Utilities|FlowControl|DoOnce false
    (:Completed
      (Utilities|FlowControl|Sequence
        (:then_0
          (Utilities|ActivateLightingPole))
        (:then_1
          (Variables|/Game/Blueprint/LevelDesign/BP_Trigger_Box_Debug.BP_Trigger_Box_Debug_C|SetIsActive? (Variables|Default|GetTrigger_BoxToActivate) true)
          (Components|Activation|Deactivate (Variables|Default|GetNiagara))
          (Components|DestroyComponent (Variables|Default|GetStaticMesh1))
          (Class|SNSNarrativeBlueprintFuncLib|EnqueueDialogue "/Game/Other/DataTables/Dialogues/DT_Ghosts_Dialogues.DT_Ghosts_Dialogues" "Abigail_4" false)
          (Class|IPlayerUtils|AddWhisper(Message) (Game|Player|GetPlayerPawn 0) (Variables|Default|GetWhisper%20Row%20Name) 1))))))

(event EventOnGhostComplete
  (Collision|SetCollisionProfileName (Variables|Default|GetTriggerCollision) "NoCollision" true :!class /Script/Engine.PrimitiveComponent)
  (Actor|Tick|SetActorTickEnabled true)
  (Rendering|Material|SetMaterial (Variables|Default|GetStaticMesh) 0 "/Game/ExternalPackages/WesterTown/Materials/Props/MI_Lantern.MI_Lantern"))

(fn ConstructionScript)

(fn SetLightVisibility
  (params (bNewVisibility :type Boolean))
  (Rendering|SetVisibility (Variables|Default|GetFire) bNewVisibility false)
  (Rendering|SetVisibility (Variables|Default|GetPointLight) bNewVisibility false))

(fn IsDebugGame?
  (return false))

(fn GetSettingsData
  (return 0))

(fn GetGameData
  (return 0))